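; BP_Key is a collectible key pickup that spins and moves vertically in the level.
; Two timelines drive KeyBase's yaw and height, both restarting whenever the rotation timeline finishes.
; Overlap by BP_Player_New calls KeyCollected on GameMode_Playstate, plays a 2D sound event and shows a collection widget that triggers its own removal.
; It then stops KeyLocation and destroys the actor.
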(event OnComponentBeginOverlap(PickUpRange)
  (params (OverlappedComponent :type Primitive%20Component%20Object%20Reference) (OtherActor :type Actor%20Object%20Reference) (OtherComp :type Primitive%20Component%20Object%20Reference) (OtherBodyIndex :type Integer) (bFromSweep :type Boolean) (SweepResult :type Hit%20Result%20Structure%20%28by%20ref%29))
  (Utilities|Casting|CastToBP_Player_New OtherActor)
  (bind _asgame_mode_playstate (Utilities|Casting|CastToGameMode_Playstate (Game|GetGameMode)))
  (Default|KeyCollected _asgame_mode_playstate)
  (Class|FMODBlueprintStatics|PlayEvent2D "/Game/FMOD/Events/UI/UI_KeyCollected.UI_KeyCollected")
  (bind _returnvalue (UserInterface|CreateWidget "/Game/UI/Player/UI_Asset_KeyCollected.UI_Asset_KeyCollected_C"))
  (UserInterface|Viewport|AddtoViewport _returnvalue 0)
  (Default|RemovefromScreen _returnvalue)
  (Class|FMODAudioComponent|Stop (Variables|Default|GetKeyLocation))
  (Actor|DestroyActor))

(event Custom|Animation
  (Utilities|FlowControl|Sequence
    (:then_0
      (bind _alpha (Timeline|RotANIM PlayFromStart)
        (:Update
          (Transformation|SetRelativeRotation (Variables|Default|GetKeyBase) (Math|Rotator|MakeRotator 0.0 0.0 (Math|Float|Lerp 0.0 359.0 _alpha)) false false))
        (:Finished
          (CallFunction|Animation))))
    (:then_1
      (bind _alpha_2 (Timeline|MoveANIM PlayFromStart)
        (:Update
          (Transformation|SetRelativeLocation (Variables|Default|GetKeyBase) (Math|Vector|MakeVector 0.0 0.0 (Math|Float|Lerp 0.0 25.0 _alpha_2)) true false))))))

(event EventBeginPlay
  (CallFunction|Animation))

(fn ConstructionScript)