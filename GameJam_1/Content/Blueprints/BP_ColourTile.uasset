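; BP_ColourTile is a puzzle floor pad in the style of Lights Out, showing blue when on and red when off.
; When BP_Player enters its TriggerBox, it flips its own IsOn state and that of every pad in AdjacentPads.
; Tick reapplies the matching material every frame.
; The Correct_SFX sound plays on any overlap, before the player class check.
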(event OnComponentBeginOverlap(TriggerBox)
  (params (OverlappedComponent :type Primitive%20Component%20Object%20Reference) (OtherActor :type Actor%20Object%20Reference) (OtherComp :type Primitive%20Component%20Object%20Reference) (OtherBodyIndex :type Integer) (bFromSweep :type Boolean) (SweepResult :type Hit%20Result%20Structure%20%28by%20ref%29))
  (Audio|PlaySound2D "/Game/Audio/SFX/WAVs/Correct_SFX.Correct_SFX" 1.0 1.0 0.0 0 0)
  (if (== (Utilities|GetClass OtherActor) "/Game/Blueprints/BP_Player.BP_Player_C")
    (if (Variables|Default|GetisOn?)
      (Variables|Default|SetisOn? false)
      (else
        (Variables|Default|SetisOn? true)))
    (for _array_element (Variables|Default|GetAdjacentPads)
      (if (Variables|BP_ColourTile_C|GetisOn? _array_element)
        (Variables|BP_ColourTile_C|SetisOn? _array_element false)
        (else
          (Variables|BP_ColourTile_C|SetisOn? _array_element true))))))

(event EventTick
  (params (DeltaSeconds :type Float%20%28single-precision%29))
  (bind _tile (Variables|Default|GetTile))
  (if (Variables|Default|GetisOn?)
    (Rendering|Material|SetMaterial _tile 0 "/Game/Assets/Materials/M_Blue.M_Blue")
    (else
      (Rendering|Material|SetMaterial _tile 0 "/Game/Assets/Materials/M_Red.M_Red"))))

(fn ConstructionScript)