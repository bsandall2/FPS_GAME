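; Game mode that runs a turn-based dice game between the player and a single BP_Enemy.
; CheckCurrentGameState drives roll and movement phases through delayed calls on both pawns, firing turn dispatchers and switching cameras; a skip flag returns play straight to the player.
; While EnemyVisible is set, player turns apply a translucent clown material to the enemy, clearing the flag after a turn count.
; DiceResults converts the rolled number to an enum and broadcasts it.
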(event Custom|Check%20Current%20Game%20State
  (params (Game%20State :type GM_States%20Enum :default "NewEnumerator0"))
  (bind _player_ref (Variables|Default|GetPlayer%20REF))
  (bind _bp_enemy (Variables|Default|GetBP%20Enemy))
  (Utilities|FlowControl|Delay 0.5)
  (switch Utilities|FlowControl|Switch|SwitchonGM_States Game%20State
    (:NewEnumerator0
      (Default|PlayersTurn _player_ref :!label _label)
      (Default|CallPlayerTurn)
      (CallFunction|CheckEnemyVisible)
      (Variables|Default|SetEnemyTurn? false)
      (Utilities|FlowControl|Delay 1.0)
      (Default|ChangetoPlayerCamera (Variables|Default|GetBP%20Enemy)))
    (:NewEnumerator2
      (Default|RollEnded _player_ref))
    (:NewEnumerator3
      (if (Variables|Default|GetTurnSkipped)
        (Variables|Default|SetTurnSkipped false)
        (goto _label)
        (else
          (Default|SpawnPather (Variables|Default|GetBP%20Enemy))
          (Default|CallEnemyTurn)
          (Variables|Default|SetEnemyTurn? true)
          (Utilities|FlowControl|Delay 1.0)
          (Default|ChangetoEnemyCamera (Variables|Default|GetPlayer%20REF)))))
    (:NewEnumerator4
      (Default|RollDice _bp_enemy))
    (:NewEnumerator6
      (Default|MovetoPlayer _bp_enemy))))

(event Custom|DiceResults
  (params (Dice%20INT :type Integer))
  (CallFunction|CheckDiceResults Dice%20INT Dice%20INT Dice%20INT Dice%20INT Dice%20INT Dice%20INT)
  (Default|CallDiceRolled))

(event Custom|SkipEnemyNextTurn
  (Variables|Default|SetTurnSkipped true))

(event Custom|CheckEnemyVisible
  (if (Variables|Default|GetEnemyVisible)
    (Utilities|FlowControl|Delay 1.0)
    (Rendering|Material|SetMaterial (Variables|/Script/Engine.Character|GetMesh (Variables|Default|GetBP%20Enemy)) 0 "/Game/Assets/Enemy/Materials/ClownTranslucent_material.ClownTranslucent_material")
    (bind _result (Math|Integer|IncrementInt (Variables|Default|GetTurnsVisible))
      (:%20%20
        (if (== _result 2)
          (Variables|Default|SetEnemyVisible false)
          (Variables|Default|SetTurnsVisible 0))))))

(event EventBeginPlay
  (Utilities|FlowControl|Sequence
    (:then_0
      (bind _asbp_player_new (Utilities|Casting|CastToBP_Player_New (Game|GetPlayerCharacter 0)))
      (Variables|Default|SetPlayer%20REF _asbp_player_new))
    (:then_1
      (bind _outactors (Actor|GetAllActorsOfClass "/Game/Blueprints/BP_Enemy.BP_Enemy_C"))
      (Variables|Default|SetBP%20Enemy (Utilities|Array|Get(acopy) _outactors)))
    (:then_2
      (CallFunction|CheckCurrentGameState "NewEnumerator0"))))

(fn ConstructionScript)

(fn CheckDiceResults
  (params (1 :type Integer) (2 :type Integer) (3 :type Integer) (4 :type Integer) (5 :type Integer) (6 :type Integer))
  (Utilities|FlowControl|Sequence
    (:then_0
      (if (== 6 1)
        (Variables|Default|SetDiceResultsENUM "NewEnumerator0")))
    (:then_1
      (if (== 1 2)
        (Variables|Default|SetDiceResultsENUM "NewEnumerator1")))
    (:then_2
      (if (== 3 3)
        (Variables|Default|SetDiceResultsENUM "NewEnumerator2")))
    (:then_3
      (if (== 2 4)
        (Variables|Default|SetDiceResultsENUM "NewEnumerator3")))
    (:then_4
      (if (== 5 5)
        (Variables|Default|SetDiceResultsENUM "NewEnumerator5")))
    (:then_5
      (if (== 4 6)
        (Variables|Default|SetDiceResultsENUM "NewEnumerator4")))))