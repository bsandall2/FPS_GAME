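; Enemy character for a turn-based dice game that hunts the player across floor tiles, reporting turn states to GameMode_Playstate.
; Its roll either moves it or, on a five, traps a random floor tile.
; A spawned BP_EnemyPather finds the player, and the enemy walks its collected tile path with AIMoveTo, one step per action.
; It also handles the kill montage, game-over screen and distance-driven reverb on footsteps and laughter.
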(event Custom|FoundPlayer
  (bind _tilestoplayerarray (Variables|Default|GetTilesToPlayerArray))
  (Utilities|Array|RemoveItem _tilestoplayerarray (Utilities|Array|Get(acopy) _tilestoplayerarray))
  (bind _asgame_mode_playstate (Utilities|Casting|CastToGameMode_Playstate (Game|GetGameMode)))
  (Default|CheckCurrentGameState _asgame_mode_playstate "NewEnumerator4"))

(event Custom|Laughing%20SFX
  (bind _laugh_event_sfx (Variables|Default|GetLaugh_Event_SFX))
  (bind _result (Math|Float|NegateFloat (/ (Transformation|GetDistanceTo (Game|GetPlayerCharacter 0)) 1e+02))
    (:%20%20
      (Class|FMODAudioComponent|SetParameter _laugh_event_sfx "Enemy Reverb" _result)
      (Class|FMODAudioComponent|Play _laugh_event_sfx))))

(event Custom|ChangeToPlayerCamera
  (bind _asbp_player_new (Utilities|Casting|CastToBP_Player_New (Game|GetPlayerCharacter 0)))
  (Game|Player|SetViewTargetwithBlend (Game|GetPlayerController 0) _asbp_player_new 0.0 "VTBlend_Linear" 0.0 false))

(event Custom|Bind%20Kill%20Event
  (bind _asbp_player_new (Utilities|Casting|CastToBP_Player_New (Game|GetPlayerCharacter 0)))
  (EventDispatchers|BindEventtoKillPlayer _asbp_player_new (delegate Custom|Kill%20Player)))

(event Custom|Kill%20Player
  (bind _returnvalue (Game|GetPlayerController 0))
  (bind _asgame_mode_playstate (Utilities|Casting|CastToGameMode_Playstate (Game|GetGameMode)))
  (Default|CheckCurrentGameState _asgame_mode_playstate "NewEnumerator8")
  (Pawn|Components|CharacterMovement|DisableMovement (Variables|Character|GetCharacterMovement))
  (Variables|Default|SetisMoving? false)
  (Game|Player|SetViewTargetwithBlend (Game|GetPlayerController 0) self 0.25 "VTBlend_EaseOut" 0.0 false)
  (Animation|Montage|PlayMontage (Variables|Character|GetMesh) "/Game/Assets/Enemy/Animations/Kill_Player_Montage.Kill_Player_Montage"
    (:then
      (Class|FMODBlueprintStatics|PlayEvent2D "/Game/FMOD/Events/Enemy/Enemy_KillPlayer.Enemy_KillPlayer"))
    (:OnCompleted
      (bind _returnvalue_2 (UserInterface|CreateWidget "/Game/UI/Menus/UI_GameOver.UI_GameOver_C"))
      (UserInterface|Viewport|AddtoViewport _returnvalue_2 0)
      (Default|GameEnded _returnvalue_2 false)
      (Input|SetInputModeUIOnly _returnvalue _returnvalue_2 "DoNotLock" false)
      (Variables|/Script/Engine.PlayerController|SetbShowMouseCursor _returnvalue true))))

(event Custom|CheckActions
  (bind _tilestoplayerarray (Variables|Default|GetTilesToPlayerArray))
  (bind _tilestoplayerarray_2 (Variables|Default|GetTilesToPlayerArray))
  (bind _output (Utilities|Array|Get(acopy) _tilestoplayerarray_2))
  (if (> (Variables|Default|GetEnemyActions) 0)
    (Utilities|IsValid _output
      (:Is%20Valid
        (AI|AIMoveTo self (Transformation|GetWorldLocation _output) 0 25.0 true
          (:then
            (Variables|Default|SetisMoving? true))
          (:OnSuccess
            (Math|Integer|DecrementInt (Variables|Default|GetEnemyActions)
              (:%20%20
                (if (> (Utilities|Array|Length _tilestoplayerarray) 0)
                  (Utilities|Array|RemoveItem _tilestoplayerarray _output)
                  (CallFunction|MovetoPlayer)))))
          (:OnFail
            (Variables|Default|SetEnemyActions 0 :!label _label)
            (CallFunction|MovetoPlayer))))
      (:Is%20Not%20Valid
        (goto _label)))
    (else
      (Variables|Default|SetisMoving? false)
      (bind _asgame_mode_playstate (Utilities|Casting|CastToGameMode_Playstate (Game|GetGameMode)))
      (Default|CheckCurrentGameState _asgame_mode_playstate "NewEnumerator0")
      (Utilities|Array|Clear (Variables|Default|GetTilesToPlayerArray))
      (Actor|DestroyActor (Variables|Default|GetPather_REF))
      (CallFunction|LaughingSFX)
      (CallFunction|StartLookingatPlayer))))

(event Custom|EnemyLight
  (params (On? :type Boolean))
  (Rendering|SetVisibility (Variables|Default|GetSpotLight) On? true))

(event Custom|MoveToPlayer
  (bind _tilestoplayerarray (Variables|Default|GetTilesToPlayerArray))
  (bind _tilestoplayerarray_2 (Variables|Default|GetTilesToPlayerArray))
  (bind _output (Utilities|Array|Get(acopy) _tilestoplayerarray_2))
  (if (or (== (Variables|Default|GetEnemyActions) 5) (== (Variables|Default|GetEnemyActions) 6))
    (Variables|Default|SetEnemyActions 0))
  (if (> (Variables|Default|GetEnemyActions) 0)
    (Utilities|IsValid _output
      (:Is%20Valid
        (AI|AIMoveTo self (Transformation|GetWorldLocation _output) 0 25.0 true
          (:then
            (Variables|Default|SetisMoving? true))
          (:OnSuccess
            (Math|Integer|DecrementInt (Variables|Default|GetEnemyActions)
              (:%20%20
                (if (> (Utilities|Array|Length _tilestoplayerarray) 0)
                  (Utilities|Array|RemoveItem _tilestoplayerarray _output)
                  (CallFunction|MovetoPlayer)))))
          (:OnFail
            (Variables|Default|SetEnemyActions 0 :!label _label)
            (CallFunction|MovetoPlayer))))
      (:Is%20Not%20Valid
        (goto _label)))
    (else
      (Variables|Default|SetisMoving? false)
      (bind _asgame_mode_playstate (Utilities|Casting|CastToGameMode_Playstate (Game|GetGameMode)))
      (Default|CheckCurrentGameState _asgame_mode_playstate "NewEnumerator0")
      (Utilities|Array|Clear (Variables|Default|GetTilesToPlayerArray))
      (Actor|DestroyActor (Variables|Default|GetPather_REF))
      (CallFunction|LaughingSFX)
      (CallFunction|StartLookingatPlayer))))

(event Custom|StartLookingAtPlayer
  (bind _returnvalue (Utilities|Time|SetTimerbyEvent (delegate Custom|LookAtPlayer) 0.5 true)))

(event Custom|RollDice
  (Variables|Default|SetEnemyActions (Math|Random|RandomIntegerinRange 1 5))
  (Class|FMODBlueprintStatics|PlayEventatLocation "/Game/FMOD/Events/Enemy/Enemy_DiceRoll.Enemy_DiceRoll" (Transformation|GetActorTransform) false)
  (Animation|Montage|PlayMontage (Variables|Character|GetMesh) "/Game/Assets/Enemy/Animations/Throw_Dice_Montage.Throw_Dice_Montage" 1.25
    (:OnCompleted
      (goto _label Reset))
    (:OnBlendOut
      (Utilities|FlowControl|DoOnce false :!label _label
        (:Completed
          (if (== (Variables|Default|GetEnemyActions) 5)
            (bind _outactors (Actor|GetAllActorsOfClass "/Game/Blueprints/BP_FloorTile.BP_FloorTile_C" :!label _label_2))
            (if (Variables|/Game/Blueprints/BP_FloorTile.BP_FloorTile_C|GetTrapCanBeSpawned (Utilities|Array|Get(acopy) _outactors (Math|Random|RandomIntegerinRange 0 (Utilities|Array|Length _outactors))))
              (Default|SpawnTrap (Utilities|Array|Get(acopy) _outactors (Math|Random|RandomIntegerinRange 0 (Utilities|Array|Length _outactors))))
              (Class|FMODBlueprintStatics|PlayEvent2D "/Game/FMOD/Events/Enemy/Enemy_PlaceTrap.Enemy_PlaceTrap")
              (bind _asgame_mode_playstate (Utilities|Casting|CastToGameMode_Playstate (Game|GetGameMode)))
              (Default|CheckCurrentGameState _asgame_mode_playstate "NewEnumerator6")
              (Default|DiceResults _asgame_mode_playstate 5 true)
              (else
                (goto _label_2)))
            (else
              (bind _asgame_mode_playstate_2 (Utilities|Casting|CastToGameMode_Playstate (Game|GetGameMode)))
              (Default|CheckCurrentGameState _asgame_mode_playstate_2 "NewEnumerator6")
              (Default|DiceResults _asgame_mode_playstate_2 (Variables|Default|GetEnemyActions) true))))))))

(event Custom|SpawnPather
  (Rendering|Material|SetMaterial (Variables|Character|GetMesh) 0 "/Game/Assets/Enemy/Materials/WhiteClown_material.WhiteClown_material")
  (Utilities|Array|Clear (Variables|Default|GetTilesToPlayerArray))
  (bind _returnvalue (Game|SpawnActorfromClass "/Game/Blueprints/BP_EnemyPather.BP_EnemyPather_C" (Transformation|GetActorTransform) "AlwaysSpawn" "MultiplyWithRoot" 0 0))
  (bind _output_get (Variables|Default|SetPather_REF _returnvalue))
  (EventDispatchers|BindEventtoPlayerFound _output_get (delegate Custom|FoundPlayer))
  (CallFunction|StopLooking))

(event Custom|LookAtPlayer
  (Transformation|SetActorRotation (Math|Interpolation|RInterpTo (Transformation|GetActorRotation) (Math|Rotator|FindLookatRotation (Transformation|GetActorLocation) (Transformation|GetActorLocation (Game|GetPlayerCharacter 0))) (Utilities|Time|GetWorldDeltaSeconds) 1e+01)))

(event Custom|StopLooking
  (Utilities|Time|ClearandInvalidateTimerbyHandle (stale Custom|StartLookingAtPlayer _returnvalue)))

(event Custom|BindFootstepEvent
  (bind _asanim_bp_enemy (Utilities|Casting|CastToANIM_BP_Enemy (Components|SkeletalMesh|GetAnimInstance (Variables|Character|GetMesh))))
  (EventDispatchers|BindEventtoFootstepSFX _asanim_bp_enemy (delegate Custom|FootstepSFX)))

(event Custom|FootstepSFX
  (bind _footstep_event_sfx (Variables|Default|GetFootstep_Event_SFX))
  (bind _result (Math|Float|NegateFloat (/ (Transformation|GetDistanceTo (Game|GetPlayerCharacter 0)) 1e+02))
    (:%20%20
      (Class|FMODAudioComponent|SetParameter _footstep_event_sfx "Enemy Reverb" _result)
      (Class|FMODAudioComponent|Play _footstep_event_sfx))))

(event EventBeginPlay
  (CallFunction|BindFootstepEvent)
  (CallFunction|BindKillEvent))

(event EventTileActivated
  (params (Floor%20Tile :type Static%20Mesh%20Component%20Object%20Reference))
  (Utilities|Array|Add (Variables|Default|GetTilesToPlayerArray) Floor%20Tile))

(fn ConstructionScript)