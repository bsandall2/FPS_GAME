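; BP_BalancePlatform is a platform actor that randomizes its own appearance and orientation when play begins.
; If CanRandomRotate is set, RotatePlaform rolls a random integer and passes it to ValueAction.
; The lowest roll hides the Platform component through visibility alone, high rolls turn RotationPoint to a 90-degree relative rotation, and the rest leave the platform unchanged.
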(event Custom|RotatePlaform
  (if (Variables|Default|GetCanRandomRotate?)
    (bind _output_get (Variables|Default|SetPlatformValue (Math|Random|RandomIntegerinRange 0 19)))
    (CallFunction|ValueAction _output_get)))

(event EventBeginPlay
  (CallFunction|RotatePlaform))

(fn ConstructionScript)

(fn ValueAction
  (params (PlatformValue :type Integer))
  (if (== PlatformValue 0)
    (Rendering|SetVisibility (Variables|Default|GetPlatform) false false)
    (elif (>= PlatformValue 11)
      (Transformation|SetRelativeRotation (Variables|Default|GetRotationPoint) "0.000000,90.000000,0.000000" false false))))