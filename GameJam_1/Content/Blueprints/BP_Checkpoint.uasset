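; BP_Checkpoint is a trigger that shuts a door and switches lights as the player passes.
; When a BP_Player overlaps its box, it clears DoorOpen on the referenced door and calls DoorCheck.
; After a delay, it sets LightIsON on the ON list and clears it on the OFF list.
; The OFF loop is nested in the ON loop, which stops after one light if the OFF list is empty.
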(event OnComponentBeginOverlap(Checkpoint_BOX)
  (params (OverlappedComponent :type Primitive%20Component%20Object%20Reference) (OtherActor :type Actor%20Object%20Reference) (OtherComp :type Primitive%20Component%20Object%20Reference) (OtherBodyIndex :type Integer) (bFromSweep :type Boolean) (SweepResult :type Hit%20Result%20Structure%20%28by%20ref%29))
  (bind _doorref (Variables|Default|GetDoorRef))
  (bind _lightsoff_ref (Variables|Default|GetLightsOFF_REF))
  (if (== (Utilities|GetClass OtherActor) "/Game/Blueprints/BP_Player.BP_Player_C")
    (Variables|/Game/Blueprints/BP_Door.BP_Door_C|SetDoorOpen _doorref false)
    (Default|DoorCheck _doorref)
    (Utilities|FlowControl|Delay 2.0)
    (bind _array_element (Utilities|Array|ForEachLoopwithBreak (Variables|Default|GetLightsON_REF))
      (:LoopBody
        (Variables|/Game/Blueprints/BP_Light.BP_Light_C|SetLight%20is%20ON _array_element true)
        (if (Utilities|Array|IsEmpty _lightsoff_ref)
          (goto _label Break)
          (else
            (bind _array_element_2 (Utilities|Array|ForEachLoopwithBreak _lightsoff_ref :!label _label)
              (:LoopBody
                (Variables|/Game/Blueprints/BP_Light.BP_Light_C|SetLight%20is%20ON _array_element_2 false)))))))))

(fn ConstructionScript)