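; BP_SecurityCamera is a security camera that turns to follow the player character and blinks its light.
; Each Tick eases LookDirection toward the player's mesh with RInterpTo, feeding a world-space rotation into SetRelativeRotation.
; Tick also calls LightChange, where a half-second Delay throttles a FlipFlop that swaps the CameraLight material between black and red.
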(event Custom|LightChange
  (bind _cameralight (Variables|Default|GetCameraLight))
  (Utilities|FlowControl|Delay 0.5)
  (Utilities|FlowControl|FlipFlop
    (:A
      (Rendering|Material|SetMaterial _cameralight 0 "/Game/Assets/Materials/M_Black.M_Black"))
    (:B
      (Rendering|Material|SetMaterial _cameralight 0 "/Game/Assets/Materials/M_Red.M_Red"))))

(event EventTick
  (params (DeltaSeconds :type Float%20%28single-precision%29))
  (bind _lookdirection (Variables|Default|GetLookDirection))
  (Transformation|SetRelativeRotation (Variables|Default|GetLookDirection) (Math|Interpolation|RInterpTo (Transformation|GetWorldRotation _lookdirection) (Math|Rotator|FindLookatRotation (Transformation|GetWorldLocation _lookdirection) (Transformation|GetWorldLocation (Variables|/Script/Engine.Character|GetMesh (Game|GetPlayerCharacter 0)))) DeltaSeconds 1.0) false false)
  (CallFunction|LightChange))

(fn ConstructionScript)