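; Physics-driven customisable die that shows the player's chosen skin and can be rolled.
; BeginPlay loads or creates the GameSave, whose skin flags select the material through SetActiveSkin; ChangeSkin passes flags directly.
; RollDice applies an upward impulse and random rotations, then a looping timer polls velocity and clears itself at rest.
; Impact audio stays gated briefly after spawn and is throttled by a delayed DoOnce reset.
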(event Custom|UpdateSkin
  (bind _gamesavefile (Variables|Default|GetGameSaveFile))
  (CallFunction|SetActiveSkin (Variables|/Game/SaveFiles/GameSave.GameSave_C|GetDC_Normal _gamesavefile) (Variables|/Game/SaveFiles/GameSave.GameSave_C|GetDC_Lit _gamesavefile) (Variables|/Game/SaveFiles/GameSave.GameSave_C|GetDC_Blood _gamesavefile) (Variables|/Game/SaveFiles/GameSave.GameSave_C|GetDC_Luck _gamesavefile) (Variables|/Game/SaveFiles/GameSave.GameSave_C|GetDC_Key _gamesavefile) (Variables|/Game/SaveFiles/GameSave.GameSave_C|GetDC_Speed _gamesavefile) (Variables|/Game/SaveFiles/GameSave.GameSave_C|GetDC_Feather _gamesavefile) (Variables|/Game/SaveFiles/GameSave.GameSave_C|GetDC_Gold _gamesavefile)))

(event Custom|CheckDiceMovement
  (if (Utilities|Operators|EqualEqual :A (Transformation|GetComponentVelocity (Variables|Default|GetDiceModel)))
    (Utilities|Time|ClearandInvalidateTimerbyHandle (stale EventRollDice _returnvalue))))

(event Custom|AllowSound
  (Utilities|FlowControl|Gate true) ; enters at Open
)

(event Collision|EventHit
  (params (MyComp :type Primitive%20Component%20Object%20Reference) (Other :type Actor%20Object%20Reference) (OtherComp :type Primitive%20Component%20Object%20Reference) (bSelfMoved :type Boolean) (HitLocation :type Vector :default "0, 0, 0") (HitNormal :type Vector :default "0, 0, 0") (NormalImpulse :type Vector :default "0, 0, 0") (Hit :type Hit%20Result%20Structure%20%28by%20ref%29))
  (Utilities|FlowControl|Gate true
    (:Exit
      (Utilities|FlowControl|DoOnce false :!label _label
        (:Completed
          (Class|FMODBlueprintStatics|PlayEventatLocation "/Game/FMOD/Events/Interactables/Dice_Impact.Dice_Impact" (Math|Conversions|ToTransform(Vector) HitLocation))
          (Utilities|FlowControl|Delay 0.75)
          (goto _label Reset))))))

(event EventBeginPlay
  (bind _returnvalue (SaveGame|DoesSaveGameExist "GameSave"))
  (if _returnvalue
    (bind _returnvalue_2 (SaveGame|LoadGamefromSlot "GameSave"))
    (bind _asgame_save (Utilities|Casting|CastToGameSave _returnvalue_2))
    (Variables|Default|SetGameSaveFile _asgame_save)
    (else
      (bind _returnvalue_3 (SaveGame|CreateSaveGameObject "/Game/SaveFiles/GameSave.GameSave_C"))
      (Variables|Default|SetGameSaveFile _returnvalue_3)))
  (CallFunction|UpdateSkin)
  (Utilities|FlowControl|Delay 2.0)
  (CallFunction|AllowSound))

(event EventRollDice
  (Utilities|FlowControl|Sequence
    (:then_0
      (Physics|AddImpulseatLocation (Variables|Default|GetDiceModel) "0.000000,0.000000,50000.000000" (Transformation|GetWorldLocation (Variables|Default|GetDiceModel)) "None")
      (for _index (range 0 30)
        (Transformation|AddLocalRotation (Variables|Default|GetDiceModel) (Math|Rotator|MakeRotator (Math|Random|RandomFloatinRange 0.0 3.6e+02) (Math|Random|RandomFloatinRange 0.0 3.6e+02) (Math|Random|RandomFloatinRange 0.0 3.6e+02)) false false)))
    (:then_1
      (bind _returnvalue (Utilities|Time|SetTimerbyEvent (delegate Custom|CheckDiceMovement) 0.1 true)))))

(event EventChangeSkin
  (params (Normal :type Boolean) (Lit :type Boolean) (Blood :type Boolean) (Luck :type Boolean) (Key :type Boolean) (Speed :type Boolean) (Feather :type Boolean) (Gold :type Boolean))
  (CallFunction|SetActiveSkin Normal Lit Blood Luck Key Speed Feather Gold))

(fn ConstructionScript
  (CallFunction|UpdateSkin))

(fn SetActiveSkin
  (params (Normal :type Boolean) (Lit :type Boolean) (Blood :type Boolean) (Luck :type Boolean) (Key :type Boolean) (Speed :type Boolean) (Feather :type Boolean) (Gold :type Boolean))
  (Utilities|FlowControl|Sequence
    (:then_0
      (if Normal
        (Rendering|Material|SetMaterial (Variables|Default|GetDiceModel) 0 "/Game/Assets/New_Meshes/Materials/Dice/M_Dice.M_Dice")))
    (:then_1
      (if Lit
        (Rendering|Material|SetMaterial (Variables|Default|GetDiceModel) 0 "/Game/Assets/New_Meshes/Materials/Dice/M_Dice_Lit.M_Dice_Lit")))
    (:then_2
      (if Blood
        (Rendering|Material|SetMaterial (Variables|Default|GetDiceModel) 0 "/Game/Assets/New_Meshes/Materials/Dice/M_Dice_Blood.M_Dice_Blood")))
    (:then_3
      (if Luck
        (Rendering|Material|SetMaterial (Variables|Default|GetDiceModel) 0 "/Game/Assets/New_Meshes/Materials/Dice/M_Dice_Luck.M_Dice_Luck")))
    (:then_4
      (if Key
        (Rendering|Material|SetMaterial (Variables|Default|GetDiceModel) 0 "/Game/Assets/New_Meshes/Materials/Dice/M_Dice_Key.M_Dice_Key")))
    (:then_5
      (if Speed
        (Rendering|Material|SetMaterial (Variables|Default|GetDiceModel) 0 "/Game/Assets/New_Meshes/Materials/Dice/M_Dice_Speed.M_Dice_Speed")))
    (:then_6
      (if Feather
        (Rendering|Material|SetMaterial (Variables|Default|GetDiceModel) 0 "/Game/Assets/New_Meshes/Materials/Dice/M_Dice_Feather.M_Dice_Feather")))
    (:then_7
      (if Gold
        (Rendering|Material|SetMaterial (Variables|Default|GetDiceModel) 0 "/Game/Assets/New_Meshes/Materials/Dice/M_Dice_Gold.M_Dice_Gold")))))