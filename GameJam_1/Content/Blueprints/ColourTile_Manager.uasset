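; ColourTile_Manager links a set of colour puzzle tiles to a door.
; On BeginPlay it binds tile events: a correct tile registers a switch on LinkedDoor, while a reset turns every tile off and resets the door, each with a sound.
; Tick compares the door's active switches to the number needed, but both branches set DoorOpen true, so the count does not gate that flag.
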(event Custom|ResetAllTiles
  (CallFunction|ResetDoorAmount)
  (for _array_element (Variables|Default|GetTiles)
    (Default|TurnOFF _array_element)))

(event Custom|CorrectSwitch
  (Default|SwitchActivated (Variables|Default|GetLinkedDoor))
  (Audio|PlaySound2D "/Game/Audio/SFX/WAVs/Correct_SFX.Correct_SFX" 1.0 1.0 0.0 0 0))

(event Custom|Reset%20Door%20Amount
  (Default|ResetDoor (Variables|Default|GetLinkedDoor))
  (Audio|PlaySound2D "/Game/Audio/SFX/WAVs/Incorrect_SFX.Incorrect_SFX" 1.0 1.0 0.0 0 0))

(event Custom|DoorAmountChecker
  (bind _linkeddoor (Variables|Default|GetLinkedDoor))
  (if (>= (Variables|/Game/Blueprints/BP_Door.BP_Door_C|GetSwitchesActive _linkeddoor) (Variables|/Game/Blueprints/BP_Door.BP_Door_C|GetSwitchesNeeded _linkeddoor))
    (Variables|/Game/Blueprints/BP_Door.BP_Door_C|SetDoorOpen _linkeddoor true)
    (else
      (Variables|/Game/Blueprints/BP_Door.BP_Door_C|SetDoorOpen _linkeddoor true))))

(event EventBeginPlay
  (bind _tiles (Variables|Default|GetTiles))
  (EventDispatchers|BindEventtoCallReset _tiles (delegate Custom|ResetAllTiles))
  (EventDispatchers|BindEventtoCallCorrect _tiles (delegate Custom|CorrectSwitch)))

(event EventTick
  (params (DeltaSeconds :type Float%20%28single-precision%29))
  (CallFunction|DoorAmountChecker))

(fn ConstructionScript)