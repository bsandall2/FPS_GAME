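; BP_Cube is a cube actor that plays a box impact sound at its location when it hits something while moving.
; Its hit event checks the hit component's speed against a small threshold, then passes through a DoOnce to play the sound.
; A short delay calls ResetSFX to re-arm the DoOnce, limiting repeated sounds, while hits at or below the threshold re-arm it immediately.
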(event OnComponentHit(Cube)
  (params (HitComponent :type Primitive%20Component%20Object%20Reference) (OtherActor :type Actor%20Object%20Reference) (OtherComp :type Primitive%20Component%20Object%20Reference) (NormalImpulse :type Vector :default "0, 0, 0") (Hit :type Hit%20Result%20Structure%20%28by%20ref%29))
  (if (> (Math|Vector|VectorLength (Transformation|GetComponentVelocity HitComponent)) 1e+01)
    (Utilities|FlowControl|DoOnce false
      (:Completed
        (Audio|PlaySoundatLocation "/Game/Audio/SFX/Box_Impact_Cue.Box_Impact_Cue" (Transformation|GetWorldLocation (Variables|Default|GetCube)) "0, 0, 0" 1.0 1.0 0.0 0 0 0 0)
        (Utilities|FlowControl|Delay 0.5)
        (CallFunction|ResetSFX)))
    (else
      (CallFunction|ResetSFX))))

(event Custom|ResetSFX
  (Utilities|FlowControl|DoOnce false) ; enters at Reset
)

(fn ConstructionScript)