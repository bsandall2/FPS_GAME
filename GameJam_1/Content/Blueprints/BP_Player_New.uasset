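; First-person player pawn for a turn-based, dice-driven horror game with tile movement, 90-degree turns and death on enemy overlap.
; On its turn it spawns a rollable BP_Dice, whose results feed card draws or skips through GameMode_Playstate.
; Gates limit timeline-driven steps to remaining actions; steps can drop a temporary mannequin decoy.
; Per-tick traces drive blocked-path UI and camera focus, while a timer points the compass at key or exit.
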(event OnComponentBeginOverlap(DiceResetBox)
  (params (OverlappedComponent :type Primitive%20Component%20Object%20Reference) (OtherActor :type Actor%20Object%20Reference) (OtherComp :type Primitive%20Component%20Object%20Reference) (OtherBodyIndex :type Integer) (bFromSweep :type Boolean) (SweepResult :type Hit%20Result%20Structure%20%28by%20ref%29))
  (bind _dicereference (Variables|Default|GetDiceReference))
  (if (== OtherActor _dicereference)
    (Actor|DestroyActor _dicereference)
    (CallFunction|ResetDice)))

(event OnComponentBeginOverlap(Sphere)
  (params (OverlappedComponent :type Primitive%20Component%20Object%20Reference) (OtherActor :type Actor%20Object%20Reference) (OtherComp :type Primitive%20Component%20Object%20Reference) (OtherBodyIndex :type Integer) (bFromSweep :type Boolean) (SweepResult :type Hit%20Result%20Structure%20%28by%20ref%29))
  (Utilities|Casting|CastToBP_Enemy OtherActor)
  (Default|CallKillPlayer))

(event Custom|Movement
  (Variables|Default|SetPreviousTrans (Transformation|GetActorTransform))
  (bind _movement_alpha (Timeline|Player%20Movement PlayFromStart)
    (:Update
      (Variables|Default|SetMovement_Ready? false)
      (CallFunction|StartFootstepsSFX)
      (Transformation|SetActorLocation (Math|Vector|Lerp(Vector) (Transformation|GetActorLocation) (Variables|Default|GetForwardBackward_Vector) _movement_alpha) true false))
    (:Finished
      (Variables|Default|SetMovement_Ready? true)
      (CallFunction|StopFootstepsSFX)
      (bind _result (Math|Integer|DecrementInt (Variables|Default|GetActions))
        (:%20%20
          (CallFunction|ActionCheck _result)
          (Utilities|FlowControl|Sequence
            (:then_0
              (if (Variables|Default|GetCanSpawnMannequin)
                (Variables|Default|SetSpawnedMannequin true)
                (bind _returnvalue (Game|SpawnActorfromClass "/Game/Blueprints/BP_Mannequin.BP_Mannequin_C" (Math|Transform|MakeTransform (- (.location (Variables|Default|GetPreviousTrans)) "0.000000,0.000000,100.000000") (Transformation|GetActorRotation) "1.000000,1.000000,1.000000") "Undefined" "MultiplyWithRoot" 0 0))
                (Variables|Default|SetCanSpawnMannequin false)
                (Class|FMODBlueprintStatics|PlayEventatLocation "/Game/FMOD/Events/Decoy/SpawnDecoy.SpawnDecoy" (Math|Transform|MakeTransform (- (.location (Variables|Default|GetPreviousTrans)) "0.000000,0.000000,100.000000") "0, 0, 0" "1.000000,1.000000,1.000000") false)))
            (:then_1
              (if (Variables|Default|GetSpawnedMannequin)
                (Math|Float|IncrementFloat (Variables|Default|GetTilesMoved)
                  (:%20%20
                    (if (== (Variables|Default|GetTilesMoved) 1e+01)
                      (Actor|DestroyActor _returnvalue)
                      (Variables|Default|SetSpawnedMannequin false)
                      (Variables|Default|SetTilesMoved 0.0))))))))))))

(event Custom|Rotation
  (bind _rotation_alpha (Timeline|Player%20Rotation PlayFromStart)
    (:Update
      (Variables|Default|SetMovement_Ready? false)
      (Pawn|SetControlRotation (Game|GetPlayerController 0) (Math|Rotator|Lerp(Rotator) (Transformation|GetActorRotation) (Variables|Default|GetLeftRight_Rotation) _rotation_alpha true)))
    (:Finished
      (Variables|Default|SetMovement_Ready? true))))

(event Custom|StartFootstepsSFX
  (Utilities|FlowControl|DoOnce false
    (:Completed
      (bind _returnvalue (Utilities|Time|SetTimerbyEvent (delegate Custom|PlayFootstepSFX) (Variables|Default|GetFootstepInterval) true)))))

(event Custom|StopFootstepsSFX
  (Utilities|Time|ClearandInvalidateTimerbyHandle (stale Custom|StartFootstepsSFX _returnvalue))
  (Utilities|FlowControl|DoOnce false) ; enters at Reset
)

(event Custom|Roll%20Ended
  (bind _springarm (Variables|Default|GetSpringArm))
  (CallFunction|DiceCollision false)
  (Utilities|FlowControl|Sequence
    (:then_0
      (Rendering|SetVisibility (Variables|Default|GetSpotLight) false false)
      (Variables|Default|SetDicePrompt false)
      (Utilities|FlowControl|Gate true) ; enters at Close
    )
    (:then_1
      (bind _camera_alpha (Timeline|CameraRotation ReverseFromEnd)
        (:Update
          (Transformation|SetRelativeLocationAndRotation _springarm (Variables|/Script/Engine.SceneComponent|GetRelativeLocation _springarm) (Math|Rotator|MakeRotator 0.0 (Math|Float|Lerp 0.0 -45.0 _camera_alpha) 0.0) false false))
        (:Finished
          (if (Variables|Default|GetPlayerBusy?)
            (Variables|Default|SetPlayerBusy? false)
            (else
              (Variables|Default|SetPlayerBusy? true))))))
    (:then_2
      (Utilities|FlowControl|Delay 0.5)
      (Actor|DestroyActor (Variables|Default|GetDiceReference)))
    (:then_3
      (CallFunction|ActionCheck (Variables|Default|GetActions)))))

(event Custom|Add%20Player%20UI
  (bind _returnvalue (UserInterface|CreateWidget "/Game/UI/Player/WID_Player_UI.WID_Player_UI_C"))
  (bind _output_get (Variables|Default|SetPlayerUIRef _returnvalue))
  (UserInterface|Viewport|AddtoViewport _output_get 0))

(event Custom|PlayerSkipped
  (CallFunction|RollEnded)
  (bind _asgame_mode_playstate (Utilities|Casting|CastToGameMode_Playstate (Game|GetGameMode)))
  (Default|CheckCurrentGameState _asgame_mode_playstate "NewEnumerator2"))

(event Custom|DiceCollision
  (params (DiceCollisionActive? :type Boolean))
  (bind _box1 (Variables|Default|GetBox1))
  (if DiceCollisionActive?
    (Rendering|SetVisibility _box1 true true)
    (else
      (Rendering|SetVisibility _box1 false true))))

(event Custom|FlashLightActive
  (params (Active :type Boolean))
  (Rendering|SetVisibility (Variables|Default|GetFlashlight) Active false))

(event Custom|Player%20Action%20Avaliable
  (Utilities|FlowControl|Sequence
    (:then_0
      (Utilities|FlowControl|Gate true) ; enters at Open
    )
    (:then_1
      (Utilities|FlowControl|Gate true) ; enters at Open
    )))

(event Custom|Out%20of%20Actions
  (Utilities|FlowControl|Sequence
    (:then_0
      (Utilities|FlowControl|Gate true) ; enters at Close
    )
    (:then_1
      (Utilities|FlowControl|Gate true) ; enters at Close
    )))

(event Custom|Compass_Begin
  (Default|ActivateCompass (Variables|Default|GetPlayerUIRef) true)
  (bind _asgame_mode_playstate (Utilities|Casting|CastToGameMode_Playstate (Game|GetGameMode)))
  (Variables|Default|SetGame%20Mode _asgame_mode_playstate)
  (bind _outactors (Actor|GetAllActorsOfClass "/Game/Blueprints/BP_ExitSign.BP_ExitSign_C"))
  (Variables|Default|SetExit_LOC (Transformation|GetActorLocation (Utilities|Array|Get(acopy) _outactors)))
  (bind _outactors_2 (Actor|GetAllActorsOfClass "/Game/Blueprints/BP_Key.BP_Key_C"))
  (Utilities|IsValid (Utilities|Array|Get(acopy) _outactors_2)
    (:Is%20Valid
      (Variables|Default|SetKey_LOC (Transformation|GetActorLocation (Utilities|Array|Get(acopy) _outactors_2))))
    (:Is%20Not%20Valid
      _))
  (Utilities|Time|SetTimerbyEvent (delegate Custom|PointCompass) 0.1 true))

(event Custom|CollisionCheck
  (bind _returnvalue (Transformation|GetActorLocation))
  (bind _returnvalue_2 (Transformation|GetActorLocation))
  (Utilities|FlowControl|Sequence
    (:then_0
      (bind _returnvalue_3 (Collision|LineTraceByChannel _returnvalue (+ _returnvalue (* (Transformation|GetActorForwardVector) 2.5e+02)) "TraceTypeQuery1" false 0 "None"))
      (bind _output_get (Variables|Default|SetForwardBlockedPath _returnvalue_3))
      (Default|DirectionUIVis (Variables|Default|GetPlayerUIRef) _output_get (stale _output_get_2)))
    (:then_1
      (bind _returnvalue_4 (Collision|LineTraceByChannel _returnvalue_2 (+ _returnvalue_2 (* (Transformation|GetActorForwardVector) -2.5e+02)) "TraceTypeQuery1" false 0 "None"))
      (bind _output_get_2 (Variables|Default|SetBackwardBlockedPath _returnvalue_4)))))

(event Custom|PointCompass
  (if (Variables|/Game/Blueprints/GameMode_Playstate.GameMode_Playstate_C|GetKeyCollected? (Variables|Default|GetGame%20Mode))
    (Class|Widget|SetRenderTransformAngle (Variables|/Game/UI/Player/WID_Player_UI.WID_Player_UI_C|GetCompass_Spinny (Variables|Default|GetPlayerUIRef)) (- (.yaw (Math|Rotator|FindLookatRotation (Transformation|GetActorLocation) (Variables|Default|GetExit_LOC))) (.yaw (Pawn|GetControlRotation :!class /Script/Engine.Pawn))) :!label _label)
    (else
      (Utilities|IsValid (Utilities|Array|Get(acopy) (stale Custom|Compass_Begin _outactors_2))
        (:Is%20Valid
          (Class|Widget|SetRenderTransformAngle (Variables|/Game/UI/Player/WID_Player_UI.WID_Player_UI_C|GetCompass_Spinny (Variables|Default|GetPlayerUIRef)) (- (.yaw (Math|Rotator|FindLookatRotation (Transformation|GetActorLocation) (Variables|Default|GetKey_LOC))) (.yaw (Pawn|GetControlRotation :!class /Script/Engine.Pawn)))))
        (:Is%20Not%20Valid
          (goto _label))))))

(event Custom|BC_CardDraw
  (bind _asgame_mode_playstate (Utilities|Casting|CastToGameMode_Playstate (Game|GetGameMode)))
  (Default|CheckCurrentGameState _asgame_mode_playstate "NewEnumerator2")
  (Utilities|FlowControl|Delay 1.5)
  (Default|CardSelection (Variables|Default|GetPlayerUIRef)))

(event Custom|Mannequin_Check
  (bind _returnvalue (Transformation|GetActorLocation))
  (bind (_outhit _returnvalue_2) (Collision|LineTraceByChannel _returnvalue (+ _returnvalue (* (Transformation|GetActorForwardVector) 1e+03)) "TraceTypeQuery1" false 0 "None"))
  (if _returnvalue_2
    (Utilities|FlowControl|DoOnce false :!label _label
      (:Completed
        (bind _asbp_mannequin (Utilities|Casting|CastToBP_Mannequin (.HitActor (Collision|BreakHitResult _outhit))))
        (Class|INTMannequin|Change(Message) _asbp_mannequin)))
    (else
      (goto _label Reset))))

(event Custom|DecoyText
  (Default|DecoyDestroyed (Variables|Default|GetPlayerUIRef)))

(event Custom|Players%20Turn
  (bind _springarm (Variables|Default|GetSpringArm))
  (CallFunction|DiceCollision true)
  (Default|CallPlayersTurn)
  (Utilities|FlowControl|Sequence
    (:then_0
      (Rendering|SetVisibility (Variables|Default|GetSpotLight) true false)
      (Utilities|FlowControl|Gate true) ; enters at Open
    )
    (:then_1
      (bind _camera_alpha (Timeline|CameraRotation PlayFromStart)
        (:Update
          (Transformation|SetRelativeLocationAndRotation _springarm (Variables|/Script/Engine.SceneComponent|GetRelativeLocation _springarm) (Math|Rotator|MakeRotator 0.0 (Math|Float|Lerp 0.0 -45.0 _camera_alpha) 0.0) false false))
        (:Finished
          (if (Variables|Default|GetPlayerBusy?)
            (Variables|Default|SetPlayerBusy? false)
            (else
              (Variables|Default|SetPlayerBusy? true))))))
    (:then_2
      (Utilities|FlowControl|Delay 0.5)
      (bind _returnvalue (Game|SpawnActorfromClass "/Game/Blueprints/BP_Dice.BP_Dice_C" (Transformation|GetWorldTransform (Variables|Default|GetDiceLOC)) "Undefined" "MultiplyWithRoot" 0 0))
      (Utilities|FlowControl|Sequence
        (:then_0
          (bind _output_get (Variables|Default|SetDiceReference _returnvalue))
          (EventDispatchers|BindEventtoOnCardDraw _output_get (delegate Custom|DrawCard))
          (EventDispatchers|BindEventtoOnPlayerSkip _output_get (delegate Custom|PlayerSkipped)))
        (:then_1
          (Utilities|FlowControl|DoOnce false) ; enters at Reset
        )
        (:then_2
          (Utilities|FlowControl|Delay 0.5)
          (Variables|Default|SetDicePrompt true))))))

(event Custom|Reset%20Dice
  (bind _returnvalue (Game|SpawnActorfromClass "/Game/Blueprints/BP_Dice.BP_Dice_C" (Transformation|GetWorldTransform (Variables|Default|GetDiceLOC)) "Undefined" "MultiplyWithRoot" 0 0))
  (Utilities|FlowControl|Sequence
    (:then_0
      (bind _output_get (Variables|Default|SetDiceReference _returnvalue))
      (EventDispatchers|BindEventtoOnCardDraw _output_get (delegate Custom|DrawCard))
      (EventDispatchers|BindEventtoOnPlayerSkip _output_get (delegate Custom|PlayerSkipped)))
    (:then_1
      (Utilities|FlowControl|DoOnce false) ; enters at Reset
    )
    (:then_2
      (Utilities|FlowControl|Delay 0.5)
      (Variables|Default|SetDicePrompt true))))

(event Custom|ActionCheck
  (params (Actions :type Integer))
  (Default|CallActionsUpdated)
  (if (> Actions 0)
    (CallFunction|PlayerActionAvaliable)
    (else
      (CallFunction|OutOfActions)
      (bind _asgame_mode_playstate (Utilities|Casting|CastToGameMode_Playstate (Game|GetGameMode)))
      (Default|CheckCurrentGameState _asgame_mode_playstate "NewEnumerator3"))))

(event Custom|DrawCard
  (bind _asgame_mode_playstate (Utilities|Casting|CastToGameMode_Playstate (Game|GetGameMode)))
  (Default|CheckCurrentGameState _asgame_mode_playstate "NewEnumerator2")
  (Utilities|FlowControl|Delay 1.5)
  (Default|CardSelection (Variables|Default|GetPlayerUIRef)))

(event Custom|ChangeToEnemyCamera
  (bind _outactors (Actor|GetAllActorsOfClass "/Game/Blueprints/BP_Enemy.BP_Enemy_C"))
  (Game|Player|SetViewTargetwithBlend (Game|GetPlayerController 0) (Utilities|Array|Get(acopy) _outactors) 0.0 "VTBlend_Linear" 0.0 false))

(event Custom|CameraFocus
  (bind _firstpersoncamera (Variables|Default|GetFirstPersonCamera))
  (bind _firstpersoncamera_2 (Variables|Default|GetFirstPersonCamera))
  (bind _returnvalue (Transformation|GetWorldLocation _firstpersoncamera))
  ;[1 1 1] Camera Focus
  (bind (_outhit _returnvalue_2) (Collision|LineTraceByChannel _returnvalue (+ _returnvalue (* (Math|Vector|GetForwardVector _firstpersoncamera) "2000.000000,2000.000000,2000.000000")) "TraceTypeQuery1" false 0 "None"))
  (if _returnvalue_2
    (Variables|/Script/CinematicCamera.CineCameraComponent|SetFocusSettings _firstpersoncamera_2 (Utilities|Struct|MakeCameraFocusSettings "Manual" (.Distance (Collision|BreakHitResult _outhit)) "(ActorToTrack=None,RelativeOffset=(X=0.000000,Y=0.000000,Z=0.000000))" true 8.0 0.0))
    (else
      (Variables|/Script/CinematicCamera.CineCameraComponent|SetFocusSettings _firstpersoncamera_2 (Utilities|Struct|MakeCameraFocusSettings "Manual" 1e+05 "(ActorToTrack=None,RelativeOffset=(X=0.000000,Y=0.000000,Z=0.000000))" true 8.0 0.0)))))

(event Custom|PlayFootstepSFX
  (Class|FMODBlueprintStatics|PlayEventatLocation "/Game/FMOD/Events/Player/Footsteps.Footsteps" (Math|Conversions|ToTransform(Vector) (- (Transformation|GetActorLocation) "0.000000,0.000000,44.000000"))))

(event Input|EnhancedActionEvents|EnhancedInputActionIA_RollDice
  (params (ActionValue :type Boolean) (ElapsedSeconds :type Float%20%28double-precision%29) (TriggeredSeconds :type Float%20%28double-precision%29) (InputAction :type Input%20Action%20Object%20Reference :default "/Game/Inputs/IA_RollDice.IA_RollDice"))
  (:Started
    (Utilities|FlowControl|DoOnce false
      (:Completed
        (Variables|Default|SetDicePrompt false)
        (Utilities|FlowControl|Gate true
          (:Exit
            (Class|INTDice|RollDice(Message) (Variables|Default|GetDiceReference))))))))

(event Input|EnhancedActionEvents|EnhancedInputActionIA_Move_Forward
  (params (ActionValue :type Boolean) (ElapsedSeconds :type Float%20%28double-precision%29) (TriggeredSeconds :type Float%20%28double-precision%29) (InputAction :type Input%20Action%20Object%20Reference :default "/Game/Inputs/IA_Move_Forward.IA_Move_Forward"))
  (:Started
    (Utilities|FlowControl|Gate true
      (:Exit
        (if (not (Variables|Default|GetPlayerBusy?))
          (if (and (Variables|Default|GetMovement_Ready?) (not (Variables|Default|GetForwardBlockedPath)))
            (Variables|Default|SetForwardBackward_Vector (+ (Transformation|GetActorLocation) (* (Transformation|GetActorForwardVector) 5e+02)))
            (CallFunction|Movement)
            (CallFunction|StartFootstepsSFX)))))))

(event Input|EnhancedActionEvents|EnhancedInputActionIA_Move_Backward
  (params (ActionValue :type Boolean) (ElapsedSeconds :type Float%20%28double-precision%29) (TriggeredSeconds :type Float%20%28double-precision%29) (InputAction :type Input%20Action%20Object%20Reference :default "/Game/Inputs/IA_Move_Backward.IA_Move_Backward"))
  (:Started
    (Utilities|FlowControl|Gate true
      (:Exit
        (if (not (Variables|Default|GetPlayerBusy?))
          (if (and (Variables|Default|GetMovement_Ready?) (not (Variables|Default|GetBackwardBlockedPath)))
            (Variables|Default|SetForwardBackward_Vector (+ (Transformation|GetActorLocation) (* (Transformation|GetActorForwardVector) -5e+02)))
            (CallFunction|Movement)
            (CallFunction|StartFootstepsSFX)))))))

(event Input|EnhancedActionEvents|EnhancedInputActionIA_Look_Left
  (params (ActionValue :type Boolean) (ElapsedSeconds :type Float%20%28double-precision%29) (TriggeredSeconds :type Float%20%28double-precision%29) (InputAction :type Input%20Action%20Object%20Reference :default "/Game/Inputs/IA_Look_Left.IA_Look_Left"))
  (:Started
    (if (and (Variables|Default|GetMovement_Ready?) (not (Variables|Default|GetPlayerBusy?)))
      (Variables|Default|SetLeftRight_Rotation (Math|Rotator|CombineRotators (Transformation|GetActorRotation) "0.000000,-90.000000,0.000000"))
      (CallFunction|Rotation))))

(event Input|EnhancedActionEvents|EnhancedInputActionIA_Look_Right
  (params (ActionValue :type Boolean) (ElapsedSeconds :type Float%20%28double-precision%29) (TriggeredSeconds :type Float%20%28double-precision%29) (InputAction :type Input%20Action%20Object%20Reference :default "/Game/Inputs/IA_Look_Right.IA_Look_Right"))
  (:Started
    (if (and (Variables|Default|GetMovement_Ready?) (not (Variables|Default|GetPlayerBusy?)))
      (Variables|Default|SetLeftRight_Rotation (Math|Rotator|CombineRotators (Transformation|GetActorRotation) "0.000000,90.000000,0.000000"))
      (CallFunction|Rotation))))

(event Input|EnhancedActionEvents|EnhancedInputActionIA_PauseGame
  (params (ActionValue :type Boolean) (ElapsedSeconds :type Float%20%28double-precision%29) (TriggeredSeconds :type Float%20%28double-precision%29) (InputAction :type Input%20Action%20Object%20Reference :default "/Game/Inputs/IA_PauseGame.IA_PauseGame"))
  (:Started
    (bind _returnvalue (UserInterface|CreateWidget "/Game/UI/Menus/UI_PauseMenu.UI_PauseMenu_C"))
    (UserInterface|Viewport|AddtoViewport _returnvalue 0)))

(event EventBeginPlay
  (Utilities|FlowControl|Sequence
    (:then_0
      (bind _asplayer_controller (Utilities|Casting|CastToPlayerController (Pawn|GetController)))
      (Utilities|IsValid (PlayerController|LocalPlayerSubsystems|GetEnhancedInputLocalPlayerSubsystem _asplayer_controller)
        (:Is%20Valid
          (Input|AddMappingContext (PlayerController|LocalPlayerSubsystems|GetEnhancedInputLocalPlayerSubsystem _asplayer_controller) "/Game/Inputs/MC_Player.MC_Player" 0 "(bIgnoreAllPressedKeysUntilRelease=True,bForceImmediately=False)"))))
    (:then_1
      (CallFunction|AddPlayerUI))
    (:then_2
      (EventDispatchers|BindEventtoDecoyDestroyed (delegate Custom|DecoyText)))))

(event EventTick
  (params (DeltaSeconds :type Float%20%28single-precision%29))
  (CallFunction|CollisionCheck)
  (CallFunction|CameraFocus)
  (CallFunction|MannequinCheck))

(fn ConstructionScript)