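; Physics-driven six-sided die that the player rolls to decide their actions for the turn.
; RollDice launches and randomly rotates the mesh, then a looping timer polls velocity until it stops.
; The highest face-marker component gives the result, which goes to GameMode_Playstate and sets player actions, triggers a card draw or skips the turn.
; Hit plays a throttled impact sound at the contact point.
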(event Custom|DiceStopped
  (Utilities|FlowControl|DoOnce false
    (:Completed
      (bind _output_get (Variables|Default|SetNumberHeight (Utilities|Array|MakeArray (.Z (Math|Vector|BreakVector (Transformation|GetWorldLocation (Variables|Default|Get1_Number)))) (.Z (Math|Vector|BreakVector (Transformation|GetWorldLocation (Variables|Default|Get2_Number)))) (.Z (Math|Vector|BreakVector (Transformation|GetWorldLocation (Variables|Default|Get3_Number)))) (.Z (Math|Vector|BreakVector (Transformation|GetWorldLocation (Variables|Default|Get4_Number)))) (.Z (Math|Vector|BreakVector (Transformation|GetWorldLocation (Variables|Default|GetDraw%20Card)))) (.Z (Math|Vector|BreakVector (Transformation|GetWorldLocation (Variables|Default|GetSkip%20Turn)))))))
      (bind _output_get_2 (Variables|Default|SetDice%20Roll%20Result (+ (.IndexOfMaxValue (Math|Float|MaxOfFloatArray _output_get)) 1)))
      (Utilities|FlowControl|Sequence
        (:then_0
          (bind _asgame_mode_playstate (Utilities|Casting|CastToGameMode_Playstate (Game|GetGameMode)))
          (Default|DiceResults _asgame_mode_playstate (Variables|Default|GetDice%20Roll%20Result) false))
        (:then_1
          (if (<= _output_get_2 4)
            (bind _asbp_player_new (Utilities|Casting|CastToBP_Player_New (Game|GetPlayerCharacter 0)))
            (bind _output_get_3 (Variables|/Game/Blueprints/BP_Player_New.BP_Player_New_C|SetActions _asbp_player_new (Variables|Default|GetDice%20Roll%20Result)))
            (Default|ActionCheck _asbp_player_new _output_get_3)
            (bind _asgame_mode_playstate_2 (Utilities|Casting|CastToGameMode_Playstate (Game|GetGameMode)))
            (Default|CheckCurrentGameState _asgame_mode_playstate_2 "NewEnumerator2")
            (elif (== _output_get_2 5)
              (Default|CallOnCardDraw)
              (bind _asbp_player_new_2 (Utilities|Casting|CastToBP_Player_New (Game|GetPlayerCharacter 0)))
              (bind _output_get_4 (Variables|/Game/Blueprints/BP_Player_New.BP_Player_New_C|SetActions _asbp_player_new_2 2))
              (Default|ActionCheck _asbp_player_new_2 _output_get_4)
              (Variables|/Game/Blueprints/BP_Player_New.BP_Player_New_C|SetPlayerBusy? _asbp_player_new_2 true)
              (elif (== _output_get_2 6)
                (Default|CallOnPlayerSkip)
                (bind _asbp_player_new_3 (Utilities|Casting|CastToBP_Player_New (Game|GetPlayerCharacter 0)))
                (bind _output_get_5 (Variables|/Game/Blueprints/BP_Player_New.BP_Player_New_C|SetActions _asbp_player_new_3 0))
                (Default|ActionCheck _asbp_player_new_3 _output_get_5)))))))))

(event Custom|CheckDiceMovement
  (if (Utilities|Operators|EqualEqual :A (Transformation|GetComponentVelocity (Variables|Default|GetDiceModel)))
    (CallFunction|DiceStopped)
    (Utilities|Time|ClearandInvalidateTimerbyHandle (stale EventRollDice _returnvalue))))

(event Collision|EventHit
  (params (MyComp :type Primitive%20Component%20Object%20Reference) (Other :type Actor%20Object%20Reference) (OtherComp :type Primitive%20Component%20Object%20Reference) (bSelfMoved :type Boolean) (HitLocation :type Vector :default "0, 0, 0") (HitNormal :type Vector :default "0, 0, 0") (NormalImpulse :type Vector :default "0, 0, 0") (Hit :type Hit%20Result%20Structure%20%28by%20ref%29))
  (Utilities|FlowControl|DoOnce false :!label _label
    (:Completed
      (Class|FMODBlueprintStatics|PlayEventatLocation "/Game/FMOD/Events/Interactables/Dice_Impact.Dice_Impact" (Math|Conversions|ToTransform(Vector) HitLocation))
      (Utilities|FlowControl|Delay 0.75)
      (goto _label Reset))))

(event EventRollDice
  (Utilities|FlowControl|Sequence
    (:then_0
      (Physics|AddImpulseatLocation (Variables|Default|GetDiceModel) "0.000000,0.000000,750.000000" (Transformation|GetWorldLocation (Variables|Default|GetDiceModel)) "None")
      (for _index (range 0 30)
        (Transformation|AddLocalRotation (Variables|Default|GetDiceModel) (Math|Rotator|MakeRotator (Math|Random|RandomFloatinRange 0.0 3.6e+02) (Math|Random|RandomFloatinRange 0.0 3.6e+02) (Math|Random|RandomFloatinRange 0.0 3.6e+02)) false false))
      (Utilities|FlowControl|Delay 0.5)
      (Utilities|FlowControl|DoOnce false) ; enters at Reset
    )
    (:then_1
      (bind _returnvalue (Utilities|Time|SetTimerbyEvent (delegate Custom|CheckDiceMovement) 0.1 true)))))

(fn ConstructionScript)