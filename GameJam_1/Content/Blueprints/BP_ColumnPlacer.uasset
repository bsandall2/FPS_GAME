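; BP_ColumnPlacer is an actor Blueprint that lays out a rectangular grid of columns.
; The Construction Script calls PlaceColumns, which runs nested loops over the ColumnsX and ColumnsY counts, with SpacingX and SpacingY setting the gaps.
; Each cell adds an instance to the Column component at zero height, so the grid is built from mesh instances instead of separate actors.
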(event Custom|Place%20Columns
  (for _index (range 0 (- (Variables|Default|GetColumns%20Y) 1))
    (for _index_2 (range 0 (- (Variables|Default|GetColumns%20X) 1))
      (Components|InstancedStaticMesh|AddInstance (Variables|Default|GetColumn) (Math|Transform|MakeTransform (Math|Vector|MakeVector (* (Math|Conversions|ToFloat(Integer) _index_2) (Variables|Default|GetSpacing%20X)) (* (Variables|Default|GetSpacing%20Y) (Math|Conversions|ToFloat(Integer) _index)) 0.0) "0, 0, 0" "1.000000,1.000000,1.000000") false))))

(fn ConstructionScript
  (CallFunction|PlaceColumns))