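; BP_Player is a first-person player pawn with movement, look, jump, physics object pickup and interaction.
; Holding PickUp line-traces from the camera and grabs the hit component with a PhysicsHandle, releasing it when the input is let go.
; While an object is held, Tick keeps the handle's target at a fixed distance in front of the camera.
; Interact sends InteractMessage to every overlapping actor implementing Interact_Interface.
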(event EventTick
  (params (DeltaSeconds :type Float%20%28single-precision%29))
  (bind _firstpersoncamera (Variables|Default|GetFirstPersonCamera))
  ;[1 1 1] Object Picked Up Location
  (if (Variables|Default|GetisHoldingObject)
    (Physics|Components|PhysicsHandle|SetTargetLocation (Variables|Default|GetPhysicsHandle) (+ (Transformation|GetWorldLocation _firstpersoncamera) (* (Math|Vector|GetForwardVector (Transformation|GetWorldRotation _firstpersoncamera)) 2.5e+02)))))

(event Input|ActionEvents|InputActionJump
  (params (Key :type Key%20Structure :default "None"))
  ;[1 1 1] Movement Inputs
  (:Pressed
    (Character|Jump))
  (:Released
    (Character|StopJumping)))

(event Input|ActionEvents|InputActionPickUp
  (params (Key :type Key%20Structure :default "None"))
  (bind _firstpersoncamera (Variables|Default|GetFirstPersonCamera))
  (bind _returnvalue (Transformation|GetWorldLocation _firstpersoncamera))
  ;[1 1 1] Pick up system
  (:Pressed
    (bind (_outhit _returnvalue_2) (Collision|LineTraceByChannel _returnvalue (+ _returnvalue (* (Math|Vector|GetForwardVector (Transformation|GetWorldRotation _firstpersoncamera)) 2.5e+02)) "TraceTypeQuery1" false 0 "None"))
    (if _returnvalue_2
      (Physics|Components|PhysicsHandle|GrabComponentatLocationwithRotation (Variables|Default|GetPhysicsHandle) (.HitComponent (Collision|BreakHitResult _outhit)) "None" (Transformation|GetWorldLocation (.HitComponent (Collision|BreakHitResult _outhit))) "0, 0, 0")
      (Variables|Default|SetisHoldingObject true)))
  (:Released
    (if (Variables|Default|GetisHoldingObject)
      (Physics|Components|PhysicsHandle|ReleaseComponent (Variables|Default|GetPhysicsHandle))
      (Variables|Default|SetisHoldingObject false))))

(event Input|ActionEvents|InputActionInteract
  (params (Key :type Key%20Structure :default "None"))
  ;[1 1 1] Interact
  (:Pressed
    (bind _array_element (Utilities|Array|ForEachLoopwithBreak (Collision|GetOverlappingActors 0 :!class /Script/Engine.Actor))
      (:LoopBody
        (if (Utilities|DoesObjectImplementInterface _array_element "/Game/Blueprints/Interact_Interface.Interact_Interface_C")
          (Class|InteractInterface|Interact(Message) _array_element))))))

(event Input|AxisEvents|InputAxisMoveForward
  (params (AxisValue :type Float%20%28single-precision%29))
  ;[1 1 1] Movement Inputs
  (Pawn|Input|AddMovementInput (Transformation|GetActorForwardVector) AxisValue false))

(event Input|AxisEvents|InputAxisMoveRight
  (params (AxisValue :type Float%20%28single-precision%29))
  ;[1 1 1] Movement Inputs
  (Pawn|Input|AddMovementInput (Transformation|GetActorRightVector) AxisValue false))

(event Input|AxisEvents|InputAxisLookHorizontal
  (params (AxisValue :type Float%20%28single-precision%29))
  ;[1 1 1] Look Inputs
  (Pawn|Input|AddControllerYawInput AxisValue))

(event Input|AxisEvents|InputAxisLookVertical
  (params (AxisValue :type Float%20%28single-precision%29))
  ;[1 1 1] Look Inputs
  (Pawn|Input|AddControllerPitchInput AxisValue))

(fn ConstructionScript)