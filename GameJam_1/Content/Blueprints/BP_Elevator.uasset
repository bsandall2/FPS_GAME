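; BP_Elevator is a one-way elevator that rises when a BP_Player_Old overlaps its trigger.
; After a short delay it enables collision on a Prevention component and calls ElevatorUP.
; A DoOnce-gated timeline lerps the base's relative Z from the BottomLOC marker to TopLOC.
; When the timeline finishes, Prevention collision is disabled and the gate resets, so the next trigger replays the ascent from the bottom.
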(event OnComponentBeginOverlap(Trigger)
  (params (OverlappedComponent :type Primitive%20Component%20Object%20Reference) (OtherActor :type Actor%20Object%20Reference) (OtherComp :type Primitive%20Component%20Object%20Reference) (OtherBodyIndex :type Integer) (bFromSweep :type Boolean) (SweepResult :type Hit%20Result%20Structure%20%28by%20ref%29))
  (Utilities|Casting|CastToBP_Player_Old OtherActor)
  (Utilities|FlowControl|Delay 0.5)
  (Collision|SetCollisionEnabled (Variables|Default|GetPrevention) "QueryAndPhysics")
  (CallFunction|ElevatorUP))

(event Custom|ElevatorUP
  (Utilities|FlowControl|DoOnce false :!label _label
    (:Completed
      (bind _elevator_track (Timeline|ElevatorTimeline PlayFromStart)
        (:Update
          (Transformation|SetRelativeLocation (Variables|Default|GetElevatorBase) (Math|Vector|MakeVector 0.0 0.0 (Math|Float|Lerp (.z (Variables|/Script/Engine.SceneComponent|GetRelativeLocation (Variables|Default|GetBottom_LOC))) (.z (Variables|/Script/Engine.SceneComponent|GetRelativeLocation (Variables|Default|GetTop_LOC))) _elevator_track)) false false))
        (:Finished
          (Collision|SetCollisionEnabled (Variables|Default|GetPrevention) "NoCollision")
          (goto _label Reset))))))

(event EventBeginPlay
  (Collision|SetCollisionEnabled (Variables|Default|GetPrevention) "NoCollision"))

(fn ConstructionScript)