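; BP_LockedBars is a bars barrier that appears on a game mode signal and is removed on another.
; On BeginPlay it hides the Bars component, disables its collision, and binds to the SpawnBars and DestroyBars events of GameMode_Playstate.
; SpawnBars makes the bars visible with query and physics collision, while DestroyBars destroys the whole actor.
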(event Custom|DestroyBars
  (Actor|DestroyActor))

(event Custom|SpawnBars
  (bind _bars (Variables|Default|GetBars))
  (Rendering|SetVisibility _bars true false)
  (Collision|SetCollisionEnabled _bars "QueryAndPhysics"))

(event EventBeginPlay
  (bind _bars (Variables|Default|GetBars))
  (Collision|SetCollisionEnabled _bars "NoCollision")
  (Rendering|SetVisibility _bars false false)
  (bind _asgame_mode_playstate (Utilities|Casting|CastToGameMode_Playstate (Game|GetGameMode)))
  (EventDispatchers|BindEventtoSpawnBars _asgame_mode_playstate (delegate Custom|SpawnBars))
  (EventDispatchers|BindEventtoDestroyBars _asgame_mode_playstate (delegate Custom|DestroyBars)))

(fn ConstructionScript)