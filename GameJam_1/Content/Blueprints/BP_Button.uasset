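; Interactable button that can spawn an object, toggle a linked door and start a timer, depending on its flags.
; Each Interact spawns at SpawnPOS, flip-flops the door's DoorOpen, animates the mesh with a timeline and plays a press sound.
; With a linked timer, a DoOnce sets StartTimer on the first press and also feeds that shared chain, so it runs twice on that press.
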(event EventInteract
  (bind _linkeddoor (Variables|Default|GetLinkedDoor))
  (bind _spawnable_object (Variables|Default|GetSpawnable%20Object))
  (bind _buttonmesh (Variables|Default|GetButtonMesh))
  (Utilities|FlowControl|Sequence
    (:then_0
      (if (Variables|Default|GetisTimerLinked?)
        (Utilities|FlowControl|DoOnce false
          (:Completed
            (Variables|/Game/Blueprints/BP_CountDownSign.BP_CountDownSign_C|SetStartTimer? (Variables|Default|GetTimerStart) true)
            (Utilities|FlowControl|Sequence :!label _label
              (:then_0
                (if (Variables|Default|GetisSpawner)
                  (Game|SpawnActorfromClass (Utilities|GetClass _spawnable_object) (Math|Conversions|ToTransform(Vector) (Transformation|GetWorldLocation (Variables|Default|GetSpawnPOS))) "Undefined" _spawnable_object 0)))
              (:then_1
                (if (Variables|Default|GetisDoor)
                  (Utilities|FlowControl|FlipFlop
                    (:A
                      (Variables|/Game/Blueprints/BP_Door.BP_Door_C|SetDoorOpen _linkeddoor true))
                    (:B
                      (Variables|/Game/Blueprints/BP_Door.BP_Door_C|SetDoorOpen _linkeddoor false)))))
              (:then_2
                (bind _buttonanim (Timeline|ButtonAnimation PlayFromStart)
                  (:Update
                    (Transformation|SetRelativeLocation _buttonmesh (Math|Vector|MakeVector 0.0 _buttonanim 0.0) false false))))
              (:then_3
                (Audio|PlaySoundatLocation "/Game/Audio/SFX/ButtonPress_Cue.ButtonPress_Cue" (Transformation|GetWorldLocation _buttonmesh) "0, 0, 0" 1.0 1.0 0.0 0 0 0 0)))))))
    (:then_1
      (goto _label))))

(fn ConstructionScript)