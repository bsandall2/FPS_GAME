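; BP_DialPuzzle is a three-dial combination puzzle that drives the DoorOpen flag on a linked door.
; An interaction event yaws the given dial left or right by a set step, then calls CheckCode without passing that dial.
; CheckCode compares a dial's relative yaw to its code entry within a tolerance and stores per-dial results.
; As wired, DoorOpen becomes true when any result fails, and false otherwise.
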(event EventInteractwithPuzzle
  (params (Component :type Primitive%20Component%20Object%20Reference) (RotateLeft :type Boolean))
  (CallFunction|Rotate Component RotateLeft))

(fn ConstructionScript)

(fn Rotate
  (params (Component :type Primitive%20Component%20Object%20Reference) (RotateLeft :type Boolean))
  (if RotateLeft
    (Transformation|AddRelativeRotation Component (Math|Rotator|MakeRotator 0.0 0.0 (* (Variables|Default|GetRotateValue) -1.0)) false false)
    (else
      (Transformation|AddRelativeRotation Component (Math|Rotator|MakeRotator 0.0 0.0 (Variables|Default|GetRotateValue)) false false)))
  (CallFunction|CheckCode))

(fn CheckCode
  (params (Componenet :type Primitive%20Component%20Object%20Reference))
  (bind _door (Variables|Default|GetDoor))
  (if (== Componenet (Variables|Default|GetDial_1))
    (LocalVariables|SetSelectedMesh 0)
    (Utilities|Array|SetArrayElem (Variables|Default|GetCodeIsGood) (LocalVariables|GetSelectedMesh) (Math|Float|NearlyEqual(Float) (Utilities|Array|Get(acopy) (Variables|Default|GetCode) (LocalVariables|GetSelectedMesh)) (.yaw (Variables|/Script/Engine.SceneComponent|GetRelativeRotation Componenet)) 1.0) :!label _label)
    (bind _array_element (Utilities|Array|ForEachLoopwithBreak (Variables|Default|GetCodeIsGood) :!label _label_2)
      (:LoopBody
        (if (not _array_element)
          (LocalVariables|SetLocalFailed true)
          (goto _label_2 Break)))
      (:Completed
        (if (LocalVariables|GetLocalFailed)
          (Variables|/Game/Blueprints/BP_Door.BP_Door_C|SetDoorOpen _door true)
          (else
            (Variables|/Game/Blueprints/BP_Door.BP_Door_C|SetDoorOpen _door false)))))
    (elif (== Componenet (Variables|Default|GetDial_2))
      (LocalVariables|SetSelectedMesh 1)
      (goto _label)
      (elif (== Componenet (Variables|Default|GetDial_3))
        (LocalVariables|SetSelectedMesh 2)
        (goto _label)))))