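; End-of-level elevator that plays the win sequence when the player overlaps its trigger.
; The overlap hides the player UI, disables movement, blends the camera to the elevator, updates the play-state game mode and plays a win sound.
; A one-shot timeline raises the elevator base between bottom and top markers, then after a delay the game-over widget shows as a win with UI-only input.
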(event OnComponentBeginOverlap(Trigger)
  (params (OverlappedComponent :type Primitive%20Component%20Object%20Reference) (OtherActor :type Actor%20Object%20Reference) (OtherComp :type Primitive%20Component%20Object%20Reference) (OtherBodyIndex :type Integer) (bFromSweep :type Boolean) (SweepResult :type Hit%20Result%20Structure%20%28by%20ref%29))
  (bind _returnvalue (Game|GetPlayerController 0))
  (bind _asbp_player_new (Utilities|Casting|CastToBP_Player_New OtherActor))
  (Widget|RemovefromParent (Variables|/Game/Blueprints/BP_Player_New.BP_Player_New_C|GetPlayerUIRef _asbp_player_new))
  (Pawn|Components|CharacterMovement|DisableMovement (Variables|/Script/Engine.Character|GetCharacterMovement _asbp_player_new))
  (Game|Player|SetViewTargetwithBlend (Game|GetPlayerController 0) self 1.0 "VTBlend_EaseOut" 1.0 false)
  (Utilities|FlowControl|Delay 1.0)
  (bind _asgame_mode_playstate (Utilities|Casting|CastToGameMode_Playstate (Game|GetGameMode)))
  (Default|CheckCurrentGameState _asgame_mode_playstate "NewEnumerator11")
  (CallFunction|ElevatorUP)
  (Class|FMODBlueprintStatics|PlayEvent2D "/Game/FMOD/Events/World/Elevator_Win_SFX.Elevator_Win_SFX")
  (Utilities|FlowControl|Delay 3.0)
  (bind _returnvalue_2 (UserInterface|CreateWidget "/Game/UI/Menus/UI_GameOver.UI_GameOver_C"))
  (UserInterface|Viewport|AddtoViewport _returnvalue_2 0)
  (Default|GameEnded _returnvalue_2 true)
  (Input|SetInputModeUIOnly _returnvalue _returnvalue_2 "DoNotLock" false)
  (Variables|/Script/Engine.PlayerController|SetbShowMouseCursor _returnvalue true))

(event Custom|ElevatorUP
  (Utilities|FlowControl|DoOnce false
    (:Completed
      (bind _elevator_track (Timeline|ElevatorTimeline PlayFromStart)
        (:Update
          (Transformation|SetRelativeLocation (Variables|Default|GetElevatorBase) (Math|Vector|MakeVector 0.0 0.0 (Math|Float|Lerp (.z (Variables|/Script/Engine.SceneComponent|GetRelativeLocation (Variables|Default|GetBottom_LOC))) (.z (Variables|/Script/Engine.SceneComponent|GetRelativeLocation (Variables|Default|GetTop_LOC))) _elevator_track)) false false))))))

(fn ConstructionScript)