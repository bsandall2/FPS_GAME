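; Spike trap for a turn-based game that catches the player and costs them their next turn.
; Once armed via SetTrapToActive, a player overlap marks them busy, plays a trap event and runs a timeline moving two spikes up and two down.
; It then zeroes the player's actions and asks GameMode_Playstate to skip their turn.
; The game mode's turn-skipped event reverses the spikes, disarms the trap and frees the player.
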(event OnComponentBeginOverlap(Player_Trap_Trigger)
  (params (OverlappedComponent :type Primitive%20Component%20Object%20Reference) (OtherActor :type Actor%20Object%20Reference) (OtherComp :type Primitive%20Component%20Object%20Reference) (OtherBodyIndex :type Integer) (bFromSweep :type Boolean) (SweepResult :type Hit%20Result%20Structure%20%28by%20ref%29))
  (bind _player (Variables|Default|GetPlayer))
  (if (Variables|Default|GetActiveTrap?)
    (if (== OtherActor (Variables|Default|GetPlayer))
      (Utilities|FlowControl|DoOnce false :!label _label
        (:Completed
          (Variables|/Game/Blueprints/BP_Player_New.BP_Player_New_C|SetPlayerBusy? (Variables|Default|GetPlayer) true)
          (Class|FMODBlueprintStatics|PlayEvent2D "/Game/FMOD/Events/World/Trap.Trap")
          (Utilities|FlowControl|Delay 1.0)
          (CallFunction|ActivateTrap)
          (Utilities|FlowControl|Delay 0.5)
          (bind _asgame_mode_playstate (Utilities|Casting|CastToGameMode_Playstate (Game|GetGameMode)))
          (Default|SkipPlayerNextTurn _asgame_mode_playstate)
          (bind _output_get (Variables|/Game/Blueprints/BP_Player_New.BP_Player_New_C|SetActions _player 0))
          (Default|ActionCheck _player _output_get)))
      (else
        (goto _label Reset)))))

(event Custom|ReverseTrap
  (bind _spike_1 (Variables|Default|GetSpike_1))
  (bind _spike_3 (Variables|Default|GetSpike_3))
  (bind _spike_2 (Variables|Default|GetSpike_2))
  (bind _spike_4 (Variables|Default|GetSpike_4))
  (bind _relativelocation (Variables|/Script/Engine.SceneComponent|GetRelativeLocation _spike_4))
  (bind _relativelocation_2 (Variables|/Script/Engine.SceneComponent|GetRelativeLocation _spike_1))
  (bind _relativelocation_3 (Variables|/Script/Engine.SceneComponent|GetRelativeLocation _spike_3))
  (bind _relativelocation_4 (Variables|/Script/Engine.SceneComponent|GetRelativeLocation _spike_2))
  (Variables|/Game/Blueprints/BP_Player_New.BP_Player_New_C|SetPlayerBusy? (Variables|Default|GetPlayer) false)
  (Variables|Default|SetActiveTrap? false)
  (bind _trap_timeline (Timeline|Trap_Movement Reverse)
    (:Update
      (Utilities|FlowControl|Sequence
        (:then_0
          (Transformation|SetRelativeLocation _spike_1 (Math|Vector|MakeVector (.x _relativelocation_2) (.y _relativelocation_2) (Math|Float|Lerp -3e+02 0.0 _trap_timeline)) false false))
        (:then_1
          (Transformation|SetRelativeLocation _spike_3 (Math|Vector|MakeVector (.x _relativelocation_3) (.y _relativelocation_3) (Math|Float|Lerp -3e+02 0.0 _trap_timeline)) false false))
        (:then_2
          (Transformation|SetRelativeLocation _spike_2 (Math|Vector|MakeVector (.x _relativelocation_4) (.y _relativelocation_4) (Math|Float|Lerp 6e+02 3e+02 _trap_timeline)) false false))
        (:then_3
          (Transformation|SetRelativeLocation _spike_4 (Math|Vector|MakeVector (.x _relativelocation) (.y _relativelocation) (Math|Float|Lerp 6e+02 3e+02 _trap_timeline)) false false))))))

(event Custom|SetTrapToActive
  (Variables|Default|SetActiveTrap? true))

(event Custom|ActivateTrap
  (bind _spike_1 (Variables|Default|GetSpike_1))
  (bind _spike_3 (Variables|Default|GetSpike_3))
  (bind _spike_2 (Variables|Default|GetSpike_2))
  (bind _spike_4 (Variables|Default|GetSpike_4))
  (bind _relativelocation (Variables|/Script/Engine.SceneComponent|GetRelativeLocation _spike_4))
  (bind _relativelocation_2 (Variables|/Script/Engine.SceneComponent|GetRelativeLocation _spike_1))
  (bind _relativelocation_3 (Variables|/Script/Engine.SceneComponent|GetRelativeLocation _spike_3))
  (bind _relativelocation_4 (Variables|/Script/Engine.SceneComponent|GetRelativeLocation _spike_2))
  (bind _trap_timeline (Timeline|Trap_Movement PlayFromStart)
    (:Update
      (Utilities|FlowControl|Sequence
        (:then_0
          (Transformation|SetRelativeLocation _spike_1 (Math|Vector|MakeVector (.x _relativelocation_2) (.y _relativelocation_2) (Math|Float|Lerp -3e+02 0.0 _trap_timeline)) false false))
        (:then_1
          (Transformation|SetRelativeLocation _spike_3 (Math|Vector|MakeVector (.x _relativelocation_3) (.y _relativelocation_3) (Math|Float|Lerp -3e+02 0.0 _trap_timeline)) false false))
        (:then_2
          (Transformation|SetRelativeLocation _spike_2 (Math|Vector|MakeVector (.x _relativelocation_4) (.y _relativelocation_4) (Math|Float|Lerp 6e+02 3e+02 _trap_timeline)) false false))
        (:then_3
          (Transformation|SetRelativeLocation _spike_4 (Math|Vector|MakeVector (.x _relativelocation) (.y _relativelocation) (Math|Float|Lerp 6e+02 3e+02 _trap_timeline)) false false))))))

(event Custom|BindTurnSkip
  (bind _asgame_mode_playstate (Utilities|Casting|CastToGameMode_Playstate (Game|GetGameMode)))
  (EventDispatchers|BindEventtoTurnhasbeenSkipped _asgame_mode_playstate (delegate Custom|ReverseTrap)))

(event EventBeginPlay
  (bind _asbp_player_new (Utilities|Casting|CastToBP_Player_New (Game|GetPlayerCharacter 0)))
  (Variables|Default|SetPlayer _asbp_player_new)
  (CallFunction|BindTurnSkip))

(fn ConstructionScript)