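; BP_CountDownSign is an in-world countdown sign that resets the player when time runs out.
; Tick calls Timer and refreshes the digit text components; a one-second Delay paces the countdown while StartTimer is set and TimerPaused is clear.
; Timer borrows across separate seconds and minute digits, though the tens-of-minutes digit is only displayed, never decremented.
; At zero it turns the text red and calls ResetPlayerEVENT on BP_Player through DoOnce.
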(event Custom|Timer
  (if (and (Variables|Default|GetStartTimer?) (not (Variables|Default|GetTimerPaused?)))
    (Utilities|FlowControl|Delay 1.0)
    (if (== (Variables|Default|GetSecond) 0)
      (if (== (Variables|Default|GetSecond_1) 0)
        (if (== (Variables|Default|GetMinute) 0)
          (Rendering|Components|TextRender|SetTextRenderColor (Variables|Default|GetDivider) (Variables|Default|GetRed_Colour))
          (Utilities|FlowControl|DoOnce false
            (:Completed
              (bind _asbp_player (Utilities|Casting|CastToBP_Player (Game|GetPlayerCharacter 0)))
              (Default|ResetPlayerEVENT _asbp_player)))
          (else
            (Variables|Default|SetSecond_1 5)
            (Variables|Default|SetSecond 9)
            (bind _result (Math|Integer|DecrementInt (Variables|Default|GetMinute))
              (:%20%20
                (Variables|Default|SetMinute _result)))))
        (else
          (Variables|Default|SetSecond 9)
          (bind _result_2 (Math|Integer|DecrementInt (Variables|Default|GetSecond_1))
            (:%20%20
              (Variables|Default|SetSecond_1 _result_2)))))
      (else
        (bind _result_3 (Math|Integer|DecrementInt (Variables|Default|GetSecond))
          (:%20%20
            (Variables|Default|SetSecond _result_3)))))))

(event EventTick
  (params (DeltaSeconds :type Float%20%28single-precision%29))
  (CallFunction|Timer)
  (CallFunction|SetMinutes)
  (CallFunction|SetSeconds))

(fn ConstructionScript)

(fn SetMinutes
  (Rendering|Components|TextRender|SetText (Variables|Default|GetMinutes) (Utilities|Text|ToText(Integer) (Variables|Default|GetMinute)))
  (Rendering|Components|TextRender|SetText (Variables|Default|GetMinutes1) (Utilities|Text|ToText(Integer) (Variables|Default|GetMinute_1))))

(fn SetSeconds
  (Rendering|Components|TextRender|SetText (Variables|Default|GetSeconds) (Utilities|Text|ToText(Integer) (Variables|Default|GetSecond)))
  (Rendering|Components|TextRender|SetText (Variables|Default|GetSeconds1) (Utilities|Text|ToText(Integer) (Variables|Default|GetSecond_1))))