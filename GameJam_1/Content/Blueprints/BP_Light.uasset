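; BP_Light is a switchable light actor whose mesh material, point light visibility and hum audio follow the LightIsON flag.
; ConstructionLight runs from the construction script, and Tick re-checks the flag every frame, calling LightON or LightOFF.
; Each branch has a DoOnce, with no reset wired, that plays a sound at the hum's location, then starts or stops the hum after a short delay.
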(event Custom|LightON
  (Rendering|Material|SetMaterial (Variables|Default|GetLightMESH) 0 "/Game/Assets/Materials/M_Light_On.M_Light_On")
  (Rendering|SetVisibility (Variables|Default|GetPointLight) true false)
  (Utilities|FlowControl|DoOnce false
    (:Completed
      (Audio|PlaySoundatLocation 0 (Transformation|GetWorldLocation (Variables|Default|GetLightHUM)) "0, 0, 0" 1.0 1.0 0.0 0 0 0 0)
      (Utilities|FlowControl|Delay 0.1)
      (Audio|Components|Audio|Play (Variables|Default|GetLightHUM) 0.0))))

(event Custom|LightOFF
  (Rendering|Material|SetMaterial (Variables|Default|GetLightMESH) 0 "/Game/Assets/Materials/M_Light_Off.M_Light_Off")
  (Rendering|SetVisibility (Variables|Default|GetPointLight) false false)
  (Utilities|FlowControl|DoOnce false
    (:Completed
      (Audio|PlaySoundatLocation 0 (Transformation|GetWorldLocation (Variables|Default|GetLightHUM)) "0, 0, 0" 1.0 1.0 0.0 0 0 0 0)
      (Utilities|FlowControl|Delay 0.1)
      (Audio|Components|Audio|Stop (Variables|Default|GetLightHUM)))))

(event Custom|ConstructionLight
  (if (Variables|Default|GetLight%20is%20ON)
    (CallFunction|LightON)
    (else
      (CallFunction|LightOFF))))

(event EventTick
  (params (DeltaSeconds :type Float%20%28single-precision%29))
  (if (Variables|Default|GetLight%20is%20ON)
    (CallFunction|LightON)
    (else
      (CallFunction|LightOFF))))

(fn ConstructionScript
  (CallFunction|ConstructionLight))