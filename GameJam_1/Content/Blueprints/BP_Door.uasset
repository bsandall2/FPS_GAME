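; BP_Door is a hinged door that toggles open and closed through Interact or SwitchActive, which ignores both the switch status and the lock.
; A timeline lerps door yaw toward a left or right angle chosen at BeginPlay, reversing to close.
; A second timeline turns the handle when opening or when locked, where a DoOnce gates retries and a locked message prints.
; CheckDoorType disables and hides the Box on non-interactable doors.
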(event Custom|DoorHandleAnim
  (if (not (Variables|Default|GetDoorOpen))
    (bind _handletime (Timeline|DoorHandleTimeline PlayFromStart)
      (:Update
        (Transformation|SetRelativeRotation (Variables|Default|GetDoorHandle) (Math|Rotator|MakeRotator 0.0 (.pitch (Math|Rotator|Lerp(Rotator) (Math|Rotator|MakeRotator 0.0 0.0 0.0) (Math|Rotator|MakeRotator 0.0 3e+01 0.0) _handletime)) 0.0) false false))
      (:Finished
        (Utilities|FlowControl|DoOnce false) ; enters at Reset
      ))))

(event Custom|SetRotationValue
  (if (Variables|Default|GetToggleDoorDirection)
    (Variables|Default|SetRotationValue (Variables|Default|GetOpenLeftValue))
    (else
      (Variables|Default|SetRotationValue (Variables|Default|GetOpenRightValue)))))

(event Custom|CheckDoorType
  (bind _box (Variables|Default|GetBox))
  (if (not (Variables|Default|GetCanInteract))
    (Components|Activation|SetActive _box false false)
    (Rendering|SetVisibility _box false false)))

(event Custom|SwitchActive
  (params (SwitchStatus :type Boolean))
  (bind _door (Variables|Default|GetDoor))
  (bind _relativerotation (Variables|/Script/Engine.SceneComponent|GetRelativeRotation _door))
  (if SwitchStatus
    _
    (else
      _))
  (if (Variables|Default|GetDoorOpen)
    (Variables|Default|SetDoorOpen false)
    (bind _door_movement (Timeline|OpeningDoor ReverseFromEnd)
      (:Update
        (Transformation|SetRelativeRotation _door (Math|Rotator|MakeRotator (.roll _relativerotation) (.pitch _relativerotation) (.yaw (Math|Rotator|Lerp(Rotator) (Math|Rotator|MakeRotator (.roll _relativerotation) (.pitch _relativerotation) 0.0) (Math|Rotator|MakeRotator (.pitch _relativerotation) (.roll _relativerotation) (Variables|Default|GetRotationValue)) _door_movement))) false false)))
    (else
      (Variables|Default|SetDoorOpen true)
      (Timeline|OpeningDoor Play))))

(event EventInteract
  (bind _door (Variables|Default|GetDoor))
  (bind _relativerotation (Variables|/Script/Engine.SceneComponent|GetRelativeRotation _door))
  (if (Variables|Default|GetCanInteract)
    (CallFunction|DoorHandleAnim)
    (if (Variables|Default|GetDoorOpen)
      (Variables|Default|SetDoorOpen false)
      (bind _door_movement (Timeline|OpeningDoor ReverseFromEnd)
        (:Update
          (Transformation|SetRelativeRotation _door (Math|Rotator|MakeRotator (.roll _relativerotation) (.pitch _relativerotation) (.yaw (Math|Rotator|Lerp(Rotator) (Math|Rotator|MakeRotator (.roll _relativerotation) (.pitch _relativerotation) 0.0) (Math|Rotator|MakeRotator (.pitch _relativerotation) (.roll _relativerotation) (Variables|Default|GetRotationValue)) _door_movement))) false false)))
      (else
        (Variables|Default|SetDoorOpen true)
        (Timeline|OpeningDoor Play)))
    (else
      (Development|PrintString "DoorIsLocked")
      (Utilities|FlowControl|DoOnce false :!label _label
        (:Completed
          (bind _handletime (Timeline|DoorHandleTimeline PlayFromStart)
            (:Update
              (Transformation|SetRelativeRotation (Variables|Default|GetDoorHandle) (Math|Rotator|MakeRotator 0.0 (.pitch (Math|Rotator|Lerp(Rotator) (Math|Rotator|MakeRotator 0.0 0.0 0.0) (Math|Rotator|MakeRotator 0.0 3e+01 0.0) _handletime)) 0.0) false false))
            (:Finished
              (goto _label Reset))))))))

(event EventBeginPlay
  (Utilities|FlowControl|Sequence
    (:then_0
      (CallFunction|SetRotationValue))))

(fn ConstructionScript)