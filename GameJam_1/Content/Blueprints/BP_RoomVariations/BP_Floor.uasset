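; BP_Floor builds a rectangular tiled room at BeginPlay, with a floor, perimeter walls and randomly placed doors.
; BasicRoom lays floor instances in a grid, then calls WallorDoor along the four edges, omitting one segment unless Origin is set.
; WallorDoor spawns BP_WallDoor actors at index-eligible slots using a seeded stream, with odds falling as Doors approaches DoorCount.
; All other slots become Wall instances, and the construction script is empty.
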(event EventBeginPlay
  (CallFunction|BasicRoom))

(fn ConstructionScript)

(fn BasicRoom
  (for _index (range 0 (- (Variables|Default|GetRoomTilesY) 1))
    (for _index_2 (range 0 (- (Variables|Default|GetRoomTilesX) 1))
      (Components|InstancedStaticMesh|AddInstance (Variables|Default|GetFloor) (Math|Transform|MakeTransform (Math|Vector|MakeVector (* _index_2 (Variables|Default|GetTileSizeX)) (* (Variables|Default|GetTileSizeY) _index) 0.0) "0, 0, 0" "1.000000,1.000000,1.000000") false)))
  (for _index_3 (range 0 (- (Variables|Default|GetRoomTilesY) 1))
    (if (or (Variables|Default|GetOrigin) (!= _index_3 0))
      (CallFunction|WallorDoor (== (/ _index_3 (Variables|Default|GetDoor%20Every)) (Variables|Default|GetDoors%20Remainder)) (Math|Vector|MakeVector 0.0 (* (Variables|Default|GetTileSizeY) _index_3) 0.0) "0, 0, 0"))
    (CallFunction|WallorDoor (== (/ _index_3 (Variables|Default|GetDoor%20Every)) (Variables|Default|GetDoors%20Remainder)) (Math|Vector|MakeVector (* (Variables|Default|GetRoomTilesX) (Variables|Default|GetTileSizeX)) (* (Variables|Default|GetTileSizeY) (Math|Conversions|ToFloat(Integer) _index_3)) 0.0) "0, 0, 0"))
  (for _index_4 (range 0 (- (Variables|Default|GetRoomTilesX) 1))
    (CallFunction|WallorDoor (== (/ _index_4 (Variables|Default|GetDoor%20Every)) (Variables|Default|GetDoors%20Remainder)) (Math|Vector|MakeVector (* (Variables|Default|GetTileSizeX) _index_4) (* (Variables|Default|GetTileSizeY) (- (Math|Conversions|ToFloat(Integer) (Variables|Default|GetRoomTilesY)) 1.0)) 0.0) "0.000000,90.000000,0.000000")
    (bind _result (Math|Float|NegateFloat (+ (Variables|Default|GetTileSizeX) 1.0))
      (:%20%20
        (CallFunction|WallorDoor (== (/ _index_4 (Variables|Default|GetDoor%20Every)) (Variables|Default|GetDoors%20Remainder)) (Math|Vector|MakeVector (* (Variables|Default|GetTileSizeX) _index_4) _result 0.0) "0.000000,90.000000,0.000000")))))

(fn WallorDoor
  (params (CanDoor :type Boolean) (Instance%20Transform%20Location :type Vector) (Instance%20Transform%20Rotation :type Rotator))
  (bind _returnvalue (Transformation|GetActorTransform))
  (bind _doorcount (Variables|Default|GetDoorCount))
  (if (and CanDoor (Class|KismetMathLibrary|RandomBoolwithWeightfromStream (Variables|Default|GetRandom%20Stream) (/ (Math|Conversions|ToFloat(Integer) (- _doorcount (Utilities|Array|Length (Variables|Default|GetDoors)))) (Math|Conversions|ToFloat(Integer) _doorcount))))
    (bind _returnvalue_2 (Game|SpawnActorfromClass "/Game/Blueprints/BP_RoomVariations/BP_WallDoor.BP_WallDoor_C" (Math|Transform|MakeTransform (Math|Transform|TransformLocation _returnvalue Instance%20Transform%20Location) (Math|Transform|TransformRotation _returnvalue Instance%20Transform%20Rotation) "1.000000,1.000000,1.000000") "Undefined" "MultiplyWithRoot" 0 0))
    (Utilities|Array|Add (Variables|Default|GetDoors) _returnvalue_2)
    (else
      (Components|InstancedStaticMesh|AddInstance (Variables|Default|GetWall) (Math|Transform|MakeTransform Instance%20Transform%20Location Instance%20Transform%20Rotation "1.000000,1.000000,1.000000") false))))