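; Sensor light actor that switches its point light and mesh material on while the player is inside either of two trigger boxes.
; Overlap flags from both boxes feed a shared check that toggles the light and a "Lights Active" audio parameter on its looping sound.
; Every tick, a multi line trace to the player counts static obstacles and scales an "Occlusion" parameter on that sound by hit count.
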(event OnComponentBeginOverlap(Trigger_Range)
  (params (OverlappedComponent :type Primitive%20Component%20Object%20Reference) (OtherActor :type Actor%20Object%20Reference) (OtherComp :type Primitive%20Component%20Object%20Reference) (OtherBodyIndex :type Integer) (bFromSweep :type Boolean) (SweepResult :type Hit%20Result%20Structure%20%28by%20ref%29))
  (Utilities|Casting|CastToBP_Player_New OtherActor)
  (Variables|Default|SetBox_1_Active true)
  (CallFunction|LightCheck))

(event OnComponentEndOverlap(Trigger_Range)
  (params (OverlappedComponent :type Primitive%20Component%20Object%20Reference) (OtherActor :type Actor%20Object%20Reference) (OtherComp :type Primitive%20Component%20Object%20Reference) (OtherBodyIndex :type Integer))
  (Utilities|Casting|CastToBP_Player_New OtherActor)
  (Variables|Default|SetBox_1_Active false)
  (CallFunction|LightCheck))

(event OnComponentBeginOverlap(Trigger_Range_2)
  (params (OverlappedComponent :type Primitive%20Component%20Object%20Reference) (OtherActor :type Actor%20Object%20Reference) (OtherComp :type Primitive%20Component%20Object%20Reference) (OtherBodyIndex :type Integer) (bFromSweep :type Boolean) (SweepResult :type Hit%20Result%20Structure%20%28by%20ref%29))
  (Utilities|Casting|CastToBP_Player_New OtherActor)
  (Variables|Default|SetBox_2_Active true)
  (CallFunction|LightCheck))

(event OnComponentEndOverlap(Trigger_Range_2)
  (params (OverlappedComponent :type Primitive%20Component%20Object%20Reference) (OtherActor :type Actor%20Object%20Reference) (OtherComp :type Primitive%20Component%20Object%20Reference) (OtherBodyIndex :type Integer))
  (Utilities|Casting|CastToBP_Player_New OtherActor)
  (Variables|Default|SetBox_2_Active false)
  (CallFunction|LightCheck))

(event Custom|LightON
  (Variables|Default|SetLight%20is%20ON true)
  (Rendering|Material|SetMaterial (Variables|Default|GetLightMESH) 0 "/Game/Assets/Materials/M_Light_On.M_Light_On")
  (Rendering|SetVisibility (Variables|Default|GetPointLight) true false))

(event Custom|LightOFF
  (Variables|Default|SetLight%20is%20ON false)
  (Rendering|Material|SetMaterial (Variables|Default|GetLightMESH) 0 "/Game/Assets/Materials/M_Light_Off.M_Light_Off")
  (Rendering|SetVisibility (Variables|Default|GetPointLight) false false))

(event Custom|LightCheck
  (bind _light_sfx (Variables|Default|GetLight_SFX))
  (if (or (Variables|Default|GetBox_1_Active) (Variables|Default|GetBox_2_Active))
    (CallFunction|LightON)
    (Class|FMODAudioComponent|SetParameter _light_sfx "Lights Active" 1.0)
    (else
      (CallFunction|LightOFF)
      (Class|FMODAudioComponent|SetParameter _light_sfx "Lights Active" 0.0))))

(event Custom|AudioOcclusion
  (bind _light_sfx (Variables|Default|GetLight_SFX))
  (Variables|Default|SetPlayer_LOC (Transformation|GetActorLocation (Variables|Default|GetPlayer)))
  (Variables|Default|SetSource_LOC (Transformation|GetActorLocation))
  (Variables|Default|SetDistance (Math|Vector|VectorLength (- (Variables|Default|GetPlayer_LOC) (Variables|Default|GetSource_LOC))))
  (bind (_outhits _returnvalue) (Class|KismetSystemLibrary|LineTraceMultiforObjects (Variables|Default|GetSource_LOC) (Variables|Default|GetPlayer_LOC) (Utilities|Array|MakeArray "ObjectTypeQuery1") false (Utilities|Array|MakeArray (Variables|Default|GetPlayer)) "None" true))
  (if _returnvalue
    (Class|FMODAudioComponent|SetParameter _light_sfx "Occlusion" (/ (* (Math|Conversions|ToFloat(Integer) (Utilities|Array|Length _outhits)) (Variables|Default|GetOcclusionValuePerHit)) 1e+02))
    (else
      (Class|FMODAudioComponent|SetParameter _light_sfx "Occlusion" 0.0))))

(event EventBeginPlay
  (CallFunction|LightOFF)
  (Class|FMODAudioComponent|Play (Variables|Default|GetLight_SFX))
  (Variables|Default|SetPlayer (Game|Player|GetPlayerPawn 0)))

(event EventTick
  (params (DeltaSeconds :type Float%20%28single-precision%29))
  (CallFunction|AudioOcclusion))

(fn ConstructionScript)