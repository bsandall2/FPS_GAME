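; BP_RandomWall is an actor that randomly decides at BeginPlay whether its wall stays in the level.
; The RandomWall event rolls an integer from 0 to 2 and passes it to NumberChecker.
; NumberChecker destroys the actor on 0, makes the Wall component and its children visible on 1, and leaves the actor unchanged on 2.
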(event Custom|RandomWall
  (CallFunction|NumberChecker (Math|Random|RandomIntegerinRange 0 2)))

(event EventBeginPlay
  (CallFunction|RandomWall))

(fn ConstructionScript)

(fn NumberChecker
  (params (NumberChosen :type Integer))
  (Utilities|FlowControl|Sequence
    (:then_0
      (if (== NumberChosen 0)
        (Actor|DestroyActor)))
    (:then_1
      (if (== NumberChosen 1)
        (Rendering|SetVisibility (Variables|Default|GetWall) true true)))))