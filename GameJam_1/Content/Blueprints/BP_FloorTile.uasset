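; Floor tile actor that hosts a trap and reports its position to the enemy during pathing.
; When a BP_EnemyPather overlaps Nav_Trigger, the tile sends its CentrePoint to the first BP_Enemy found in the level.
; SpawnTrap shows and activates the child-actor trap if allowed, otherwise hides and disables it.
; On BeginPlay it binds DeactivateTrap to the GameMode_Playstate turn-skipped event, reusing that disable path.
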(event OnComponentBeginOverlap(Nav_Trigger)
  (params (OverlappedComponent :type Primitive%20Component%20Object%20Reference) (OtherActor :type Actor%20Object%20Reference) (OtherComp :type Primitive%20Component%20Object%20Reference) (OtherBodyIndex :type Integer) (bFromSweep :type Boolean) (SweepResult :type Hit%20Result%20Structure%20%28by%20ref%29))
  (Utilities|Casting|CastToBP_EnemyPather OtherActor)
  (bind _outactors (Actor|GetAllActorsOfClass "/Game/Blueprints/BP_Enemy.BP_Enemy_C"))
  (Class|INTAddTiles|TileActivated(Message) (Utilities|Array|Get(acopy) _outactors) (Variables|Default|GetCentrePoint)))

(event Custom|SpawnTrap
  (bind _trap (Variables|Default|GetTrap))
  (bind _childactor (Variables|/Script/Engine.ChildActorComponent|GetChildActor _trap))
  (if (Variables|Default|GetTrapCanBeSpawned)
    (Rendering|SetVisibility _trap true true)
    (bind _asbp_trap (Utilities|Casting|CastToBP_Trap _childactor))
    (Default|SetTraptoActive _asbp_trap)
    (else
      (Rendering|SetVisibility _trap false true)
      (bind _asbp_trap_2 (Utilities|Casting|CastToBP_Trap _childactor))
      (Variables|/Game/Blueprints/BP_Trap.BP_Trap_C|SetActiveTrap? _asbp_trap_2 false))))

(event Custom|DeactivateTrap
  (bind _trap (Variables|Default|GetTrap))
  (Rendering|SetVisibility _trap false true)
  (bind _asbp_trap (Utilities|Casting|CastToBP_Trap (Variables|/Script/Engine.ChildActorComponent|GetChildActor _trap)))
  (Variables|/Game/Blueprints/BP_Trap.BP_Trap_C|SetActiveTrap? _asbp_trap false))

(event EventBeginPlay
  (bind _asgame_mode_playstate (Utilities|Casting|CastToGameMode_Playstate (Game|GetGameMode)))
  (EventDispatchers|BindEventtoTurnhasbeenSkipped _asgame_mode_playstate (delegate Custom|DeactivateTrap)))

(fn ConstructionScript)