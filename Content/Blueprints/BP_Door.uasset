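; BP_Door is a sliding door that opens vertically when DoorOpen is set and enough switches are active.
; Switch activate, deactivate and reset events update the count and run DoorCheck, which also runs every Tick.
; DoorCheck swaps green or red materials and plays or reverses a timeline moving the mesh.
; Timeline events use a direction flag to play open or close sounds, with opening also calling ResetUIHidden on the player.
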(event Custom|SwitchDeactivated
  (bind _result (Math|Integer|DecrementInt (Variables|Default|GetSwitchesActive))
    (:%20%20
      (Variables|Default|SetSwitchesActive _result)
      (CallFunction|DoorCheck))))

(event Custom|DoorCheck
  (bind _door (Variables|Default|GetDoor))
  (bind _door_2 (Variables|Default|GetDoor))
  (bind _returnvalue (Transformation|GetWorldLocation _door_2))
  (if (> (Variables|Default|GetSwitchesNeeded) 0)
    (if (>= (Variables|Default|GetSwitchesActive) (Variables|Default|GetSwitchesNeeded))
      (if (Variables|Default|GetDoorOpen) :!label _label
        (Variables|Default|SetDoorSFX false)
        (Rendering|Material|SetMaterial _door 0 "/Game/Assets/Materials/M_Door_Green.M_Door_Green")
        (bind _door_movement (Timeline|OpeningDoor Play)
          (:Update
            (Transformation|SetRelativeLocation (Variables|Default|GetDoor) (Math|Vector|MakeVector 0.0 0.0 _door_movement) false false))
          (:PlayOpenSFX
            (if (not (Variables|Default|GetDoorSFX))
              (Audio|PlaySoundatLocation "/Game/Audio/SFX/DoorOpen_Cue.DoorOpen_Cue" _returnvalue "0, 0, 0" 1.0 1.0 0.0 0 0 0 0)
              (bind _asbp_player (Utilities|Casting|CastToBP_Player (Game|GetPlayerCharacter 0)))
              (Default|ResetUIHidden _asbp_player)))
          (:PlayCloseSFX
            (if (Variables|Default|GetDoorSFX)
              (Audio|PlaySoundatLocation "/Game/Audio/SFX/DoorClose_Cue.DoorClose_Cue" _returnvalue "0, 0, 0" 1.0 1.0 0.0 0 0 0 0))))
        (else
          (Variables|Default|SetDoorSFX true :!label _label_2)
          (Rendering|Material|SetMaterial _door 0 "/Game/Assets/Materials/M_Door_Red.M_Door_Red")
          (Timeline|OpeningDoor Reverse)))
      (else
        (goto _label_2)))
    (else
      (goto _label))))

(event Custom|SwitchActivated
  (bind _result (Math|Integer|IncrementInt (Variables|Default|GetSwitchesActive))
    (:%20%20
      (Variables|Default|SetSwitchesActive _result)
      (CallFunction|DoorCheck))))

(event Custom|ResetDoor
  (Variables|Default|SetSwitchesActive 0)
  (CallFunction|DoorCheck))

(event EventTick
  (params (DeltaSeconds :type Float%20%28single-precision%29))
  (CallFunction|DoorCheck))

(fn ConstructionScript)